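; BP_River2 is a river actor that builds deformed spline meshes along its River spline in the construction script.
; Each spline point spawns a segment using local locations and tangents toward the next point.
; Per-point Xlength entries, padded with 1.0, set segment width, with each value shared by adjoining start and end scales for continuity.
; The event graph is empty.
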(fn `UserConstructionScript`
  (locals (NewLocalVar :type "SplineComponent Object Reference"))
  (bind _splinemeshes (`self.SplineMeshes`))
  (bind _river (`self.River`))
  (bind _xlength (`self.Xlength`))
  (bind _returnvalue (`SplineComponent.GetNumberOfSplinePoints` (`self.River`)))
  (bind _returnvalue_2 (- _returnvalue 1))
  (bind _returnvalue_3 (- (`KismetArrayLibrary.Array_Length` (`self.Xlength`)) 1))
  (`KismetArrayLibrary.Array_Clear` (`self.SplineMeshes`))
  (if (> _returnvalue_2 _returnvalue_3)
    (for _index (range _returnvalue (+ _returnvalue_3 1))
      (`KismetArrayLibrary.Array_Remove` (`self.Xlength`) _index)))
  (for _index_2 (range (+ _returnvalue_2 1))
    (bind _returnvalue_4 (`AddComponent|NODE_AddSplineMeshComponent-0`))
    (`KismetArrayLibrary.Array_Add` (`self.SplineMeshes`) _returnvalue_4)
    (bind (_location _tangent) (`SplineComponent.GetLocationAndTangentAtSplinePoint` _river _index_2 "Local"))
    (bind (_location_2 _tangent_2) (`SplineComponent.GetLocationAndTangentAtSplinePoint` _river (+ _index_2 1) "Local"))
    (`SplineMeshComponent.SetStartAndEnd` _returnvalue_4 _location _tangent _location_2 _tangent_2 true)
    (`SceneComponent.K2_AttachToComponent` _returnvalue_4 (`self.DefaultSceneRoot`) "None" "KeepRelative" "KeepRelative" "KeepRelative" true)
    (if (not (`KismetArrayLibrary.Array_IsValidIndex` _xlength _index_2))
      (`KismetArrayLibrary.Array_Add` _xlength 1.0))
    (if (== _index_2 0)
      (bind _output (`|GetArrayItem` (`self.Xlength`) _index_2))
      (`SplineMeshComponent.SetStartScale` _returnvalue_4 (`KismetMathLibrary.MakeVector2D` _output 1.0) true)
      (else
        (`SplineMeshComponent.SetStartScale` (`|GetArrayItem` _splinemeshes _index_2) (`KismetMathLibrary.MakeVector2D` _output 1.0) true)
        (`SplineMeshComponent.SetEndScale` (`|GetArrayItem` _splinemeshes (- _index_2 1)) (`KismetMathLibrary.MakeVector2D` _output 1.0) true)))))