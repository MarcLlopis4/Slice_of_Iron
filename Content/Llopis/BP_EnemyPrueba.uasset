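; BP_EnemyPrueba is a test enemy character that detects BP_Maria and takes damage.
; Pawn sensing sets PlayerSeen and starts a TimeToLostPlayer timer, refreshed on each sighting, that clears the flag when it expires.
; AnyDamage subtracts from Life, with hit animation and death only stubbed as debug prints.
; A helper function sets the max walk speed; this Blueprint's graphs contain no movement or attack logic.
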(event `self.ReceiveTick`
  (params (DeltaSeconds :type "Float (single-precision)")))

(event `self.PawnSensing.OnSeePawn`
  (params (Pawn :type "Pawn Object Reference"))
  (cast `/Game/ThirdPerson/Blueprints/BP_Maria` Pawn)
  (`KismetSystemLibrary.K2_ClearTimer` null "Unsee_player")
  (set `self.playerSeen` true)
  (`KismetSystemLibrary.K2_SetTimerDelegate` (delegate `Unsee_player`) (`self.timeToLostPlayer`)))

(event `Unsee_player`
  (`KismetSystemLibrary.PrintString` "player not seen")
  (set `self.playerSeen` false))

(event `self.ReceiveAnyDamage`
  (params (Damage :type "Float (single-precision)") (DamageType :type "DamageType Object Reference") (InstigatedBy :type "Controller Object Reference") (DamageCauser :type "Actor Object Reference"))
  ; Añadir animación de hit con método para detectar frames de invulnerabilidad
  (if (<= (- (`self.life`) Damage) 0.0)
    (`KismetSystemLibrary.PrintString` "muerte")
    (else
      (`KismetSystemLibrary.PrintString` "hit animation")
      (set `self.life` (- (`self.life`) Damage)))))

(fn `SetCharacterMovementSpeed`
  (params (Speed :type "Float (double-precision)"))
  (set `CharacterMovementComponent.MaxWalkSpeed` Speed (`self.CharacterMovement`)))

(fn `UserConstructionScript`)