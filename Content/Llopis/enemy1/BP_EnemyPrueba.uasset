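; Test melee enemy character that senses BP_Ingothar, forgetting them after a timeout, and punches with Niagara effects, sound and a zero-damage hit call.
; Sword-tagged overlaps trigger damage, montages and a physics impulse.
; Tick drains Life by delta time; at zero, Death has the player's inventory component drop weighted loot, then destroys the enemy.
; Local DropItems and CheckItemToDrop hold similar weighted spawn logic, uncalled here.
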(event `CheckItemToDrop`
  (params (`Number Drops` :type Integer))
  (for _ (range `Number Drops`)
    (bind _output_get (set `self.TempItemFloat` (`KismetMathLibrary.RandomFloatInRange` 0.0 100.0)))
    (`KismetSystemLibrary.PrintString` (`KismetStringLibrary.Conv_DoubleToString` _output_get) true true (struct :`R` 1.0 :`G` 0.027768 :`A` 1.0) 10.0)
    (if (>= (`self.TempItemFloat`) (`.Value` (`BlueprintMapLibrary.Map_GetKeyValueByIndex` (`self.PullItems`))))
      (if (>= (`self.TempItemFloat`) (+ (`.Value` (`BlueprintMapLibrary.Map_GetKeyValueByIndex` (`self.PullItems`))) (`.Value` (`BlueprintMapLibrary.Map_GetKeyValueByIndex` (`self.PullItems`) 1))))
        ;[0.04438 0.1131 0.15 0.5 40] DROP EMPUÑADURA
        (`KismetSystemLibrary.PrintString` "drop empuñaduras" true true (struct :`G` 0.66 :`B` 1.0 :`A` 1.0) 10.0)
        (`|SpawnActorFromClass` "/Game/Krosty/Inventory/Blueprints/BP_ItemPartesArmas.BP_ItemPartesArmas_C" (`SceneComponent.K2_GetComponentToWorld` (`self.CapsuleComponent`)) "Undefined" "MultiplyWithRoot" null (make `/Game/Krosty/Inventory/Blueprints/S_PartesArmasStruct` "Empuñadura1" true 1 "NewEnumerator0" "/Game/Llopis/textures/HandlePNG.HandlePNG" "/Game/Llopis/Modelado_Sergi/Armas/Dagger/Handle/S_DH_Horn.S_DH_Horn") null)
        (else
          ;[0.15 0.05602 0.05251 0.5 40] DROP HOJA
          (`KismetSystemLibrary.PrintString` "drop hoja" true true (struct :`G` 0.66 :`B` 1.0 :`A` 1.0) 10.0)
          (`|SpawnActorFromClass` "/Game/Krosty/Inventory/Blueprints/BP_ItemPartesArmas.BP_ItemPartesArmas_C" (`SceneComponent.K2_GetComponentToWorld` (`self.CapsuleComponent`)) "Undefined" "MultiplyWithRoot" null (make `/Game/Krosty/Inventory/Blueprints/S_PartesArmasStruct` "Hoja1" true 1 "NewEnumerator0" "/Game/Llopis/UI/Sword.Sword" "/Game/Llopis/Modelado_Sergi/Armas/Dagger/Edge/S_DE_Snake.S_DE_Snake") null)))
      (else
        ;[0.07389 0.15 0.06369 0.5 40] DROP MATERIAL
        (`KismetSystemLibrary.PrintString` "drop Material" true true (struct :`G` 0.66 :`B` 1.0 :`A` 1.0) 10.0)
        (`|SpawnActorFromClass` "/Game/Krosty/Inventory/Blueprints/BP_ItemMaterial.BP_ItemMaterial_C" (`SceneComponent.K2_GetComponentToWorld` (`self.CapsuleComponent`)) "Undefined" "MultiplyWithRoot" null (make `/Game/Krosty/Inventory/Blueprints/S_ItemMaterialStruct` "Material1" true 1 "/Engine/EditorMaterials/Anchor.Anchor" "/Engine/BasicShapes/Cone.Cone") null)))))

(event `DropItems`
  (bind _output_get (set `self.tempNumberFloat` (`KismetMathLibrary.RandomFloatInRange` 0.0 100.0)))
  (`KismetSystemLibrary.PrintString` (`KismetStringLibrary.Conv_DoubleToString` _output_get) true true (struct :`G` 0.107302 :`B` 1.0 :`A` 1.0) 10.0)
  (if (>= (`self.tempNumberFloat`) (`.Value` (`BlueprintMapLibrary.Map_GetKeyValueByIndex` (`self.NumberItemsDroped`))))
    (if (>= (`self.tempNumberFloat`) (+ (`.Value` (`BlueprintMapLibrary.Map_GetKeyValueByIndex` (`self.NumberItemsDroped`))) (`.Value` (`BlueprintMapLibrary.Map_GetKeyValueByIndex` (`self.NumberItemsDroped`) 1))))
      ;[0.04438 0.1131 0.15 0.5 40] DROP 0
      (`KismetSystemLibrary.PrintString` "drop 0")
      (else
        ;[0.15 0.05602 0.05251 0.5 40] DROP 1
        (`KismetSystemLibrary.PrintString` "drop 1")
        (`self.CheckItemToDrop` 1)))
    (else
      ;[0.07389 0.15 0.06369 0.5 40] DROP 2
      (`KismetSystemLibrary.PrintString` "drop 2")
      (`self.CheckItemToDrop` 2))))

(event `self.ReceiveTick`
  (params (DeltaSeconds :type "Float (single-precision)"))
  (bind _output_get (set `self.life` (- (`self.life`) DeltaSeconds)))
  (if (<= _output_get 0.0)
    (`/Engine/EditorBlueprintResources/StandardMacros.DoOnce` false
      (:`Completed`
        (`self.Death`)))))

(event `self.PawnSensing.OnSeePawn`
  (params (Pawn :type "Pawn Object Reference"))
  (if (not (`self.dead`))
    (cast `/Game/ThirdPerson/Blueprints/BP_Ingothar` Pawn)
    (`KismetSystemLibrary.K2_ClearTimer` null "Unsee_player")
    (set `self.playerSeen` true)
    (`KismetSystemLibrary.K2_SetTimerDelegate` (delegate `Unsee_player`) (`self.timeToLostPlayer`))))

(event `Unsee_player`
  (`KismetSystemLibrary.PrintString` "player not seen")
  (set `self.playerSeen` false))

(event `ItemInFloor`)

(event `Death`
  (bind _asbp_ingothar (cast `/Game/ThirdPerson/Blueprints/BP_Ingothar` (`GameplayStatics.GetPlayerCharacter` 0)))
  (`/Game/Krosty/Blueprints/BP_InventoryComponent.DropItems` (`/Game/ThirdPerson/Blueprints/BP_Ingothar.BP_InventoryComponent` _asbp_ingothar) (`self.NumberItemsDroped`) (`self.PullItems`) (`self.K2_GetActorLocation`))
  (`KismetSystemLibrary.Delay` 0.2)
  (`self.K2_DestroyActor`)
  (`KismetSystemLibrary.CollectGarbage`))

(event `TakeDamage`
  (params (Damage :type "Float (double-precision)"))
  (bind _charactermovement (`self.CharacterMovement`))
  ; Añadir animación de hit con método para detectar frames de invulnerabilidad
  (if (and (not (`self.dead`)) (<= (- (`self.life`) Damage) 0.0))
    (set `self.dead` true)
    (`KismetSystemLibrary.PrintString` "dead animation")
    (`|PlayMontage` (`self.Mesh`) "/Game/Llopis/enemy1/Dying_Backwards_Montage.Dying_Backwards_Montage"
      (:`then`
        (`KismetSystemLibrary.PrintString` "updating dead")))
    (else
      (`KismetSystemLibrary.PrintString` "hit animation")
      (set `self.hit` true)
      (`|PlayMontage` (`self.Mesh`) "/Game/Llopis/enemy1/Big_Stomach_Hit_Montage.Big_Stomach_Hit_Montage"
        (:`then`
          (`CharacterMovementComponent.DisableMovement` _charactermovement)
          (set `self.life` (- (`self.life`) Damage)))
        (:`OnCompleted`
          (set `self.hit` false)
          (`PrimitiveComponent.SetSimulatePhysics` (`self.CapsuleComponent`) false)
          (`CharacterMovementComponent.SetMovementMode` _charactermovement "MOVE_Walking" 0))))))

(event `self.PunchCollider.OnComponentBeginOverlap`
  (params (OverlappedComponent :type "PrimitiveComponent Object Reference") (OtherActor :type "Actor Object Reference") (OtherComp :type "PrimitiveComponent Object Reference") (OtherBodyIndex :type Integer) (bFromSweep :type Boolean) (SweepResult :type "HitResult Structure (by ref)"))
  (bind _returnvalue (`SceneComponent.K2_GetComponentLocation` (`self.PunchCollider`)))
  (bind _asbp_ingothar (cast `/Game/ThirdPerson/Blueprints/BP_Ingothar` OtherActor))
  (`/Game/ThirdPerson/Blueprints/BP_Ingothar.TakeDamage` _asbp_ingothar 0.0 false)
  (`NiagaraFunctionLibrary.SpawnSystemAtLocation` "/Game/Llopis/Effects/BloodSys.BloodSys" _returnvalue (struct) (2.0 2.0 2.0))
  (`NiagaraFunctionLibrary.SpawnSystemAtLocation` "/Game/Llopis/enemy1/HondoChoque.HondoChoque" _returnvalue)
  (`GameplayStatics.PlaySound2D` "/Game/Llopis/enemy1/Punch.Punch" 1.0 1.0 0.0 null null))

(event `self.CapsuleComponent.OnComponentBeginOverlap`
  (params (OverlappedComponent :type "PrimitiveComponent Object Reference") (OtherActor :type "Actor Object Reference") (OtherComp :type "PrimitiveComponent Object Reference") (OtherBodyIndex :type Integer) (bFromSweep :type Boolean) (SweepResult :type "HitResult Structure (by ref)"))
  (`KismetSystemLibrary.PrintString` "begin overlappping")
  (if (and (not (`self.dead`)) (== "Sword" (`|GetArrayItem` (`ActorComponent.ComponentTags` OtherComp))))
    (`self.TakeDamage` 20.0)
    (`PrimitiveComponent.SetSimulatePhysics` (`self.CapsuleComponent`) true)
    (bind _asbp_ingothar (cast `/Game/ThirdPerson/Blueprints/BP_Ingothar` OtherActor))
    (bind (_returnvalue_x _returnvalue_y) (`KismetMathLibrary.BreakVector` (`KismetMathLibrary.GetDirectionUnitVector` (`self.K2_GetActorLocation`) (`self.K2_GetActorLocation` _asbp_ingothar))))
    (`PrimitiveComponent.AddImpulse` (`self.CapsuleComponent`) (* (`KismetMathLibrary.MakeVector` _returnvalue_x _returnvalue_y) 1000000.0) "None" false)))

(fn `SetCharacterMovementSpeed`
  (params (Speed :type "Float (double-precision)"))
  (set `CharacterMovementComponent.MaxWalkSpeed` Speed (`self.CharacterMovement`)))

(fn `UserConstructionScript`)