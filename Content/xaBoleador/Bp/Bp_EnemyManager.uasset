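; Enemy manager that records enemies and rebuilds the roster on respawn.
; RegistrarEnemy, gated by RegistroEnemy, stores each enemy with a spawn snapshot of class, transform and patrol points.
; Respawn destroys live enemies, spawns replacements from the snapshots and turns registration off.
; It also copies drop chance and item pool fields onto replacements, though RegistrarEnemy never fills those fields.
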(fn `Prueba1`
  (params (damage :type "Float (double-precision)")))

(fn `RegistrarEnemy`
  (params (Enemy :type "/Game/xaBoleador/Bp/Bp_Enemy_Base Object Reference"))
  (if (`self.registro enemy`)
    (`KismetArrayLibrary.Array_Add` (`self.Enemy_List`) Enemy)
    (`KismetArrayLibrary.Array_Add` (`self.SpawnDataList`) (make `/Game/xaBoleador/Structs_No_armas/S_enemy_Spawn` (`GameplayStatics.GetObjectClass` Enemy) (`self.K2_GetActorLocation` Enemy) (`self.K2_GetActorRotation` Enemy) (`/Game/xaBoleador/Bp/Bp_Enemy_Base.PatrolPointsPadre` Enemy) (`self.GetActorScale3D` Enemy)))))

(fn `Respawn`
  (for _array_element (`self.Enemy_List`)
    (`/Engine/EditorBlueprintResources/StandardMacros.IsValid` _array_element
      (:`Is Valid`
        (`self.K2_DestroyActor` _array_element))))
  (`KismetArrayLibrary.Array_Clear` (`self.Enemy_List`))
  (for _array_element_2 (`self.SpawnDataList`)
    (bind (_enemyclass _spawnlocationactor _spawnrotation _patrolpoints _scale _probtiempull _objectspull _filospull _mangospull _materialespull) (break `/Game/xaBoleador/Structs_No_armas/S_enemy_Spawn` _array_element_2))
    (bind _returnvalue (`|SpawnActorFromClass` _enemyclass (`KismetMathLibrary.MakeTransform` _spawnlocationactor _spawnrotation) "Undefined" "MultiplyWithRoot" null null))
    (`self.SetActorScale3D` _returnvalue _scale)
    (`KismetArrayLibrary.Array_Add` (`self.Enemy_List`) _returnvalue)
    (set `self.registro enemy` false)
    (set `/Game/xaBoleador/Bp/Bp_Enemy_Base.PatrolPointsPadre` _patrolpoints _returnvalue)
    (set `/Game/xaBoleador/Bp/Bp_Enemy_Base.ProbItemsDroppedPadre` _probtiempull _returnvalue)
    (set `/Game/xaBoleador/Bp/Bp_Enemy_Base.ObjectsPullpadre` _objectspull _returnvalue)
    (set `/Game/xaBoleador/Bp/Bp_Enemy_Base.FilosPullPadre` _filospull _returnvalue)
    (set `/Game/xaBoleador/Bp/Bp_Enemy_Base.MangosPullPadre` _mangospull _returnvalue)
    (set `/Game/xaBoleador/Bp/Bp_Enemy_Base.MaterialesPullPadre` _materialespull _returnvalue)))

(fn `UserConstructionScript`)