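; Shop actor selling armor, weapon parts, materials and key items to BP_Ingothar, registered as the player's CurrentTienda while inside its box.
; BeginPlay caches the player's inventory component and fills four stock arrays from DataTables.
; Per-category TryBuy functions deduct the price from GameInstance currency and decrement stock.
; Separate Repasar events add items to inventory, stacking by name up to 64 or using an empty slot, then refresh the widget.
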(event `self.ReceiveBeginPlay`
  (bind _asbp_ingothar (cast `/Game/ThirdPerson/Blueprints/BP_Ingothar` (`GameplayStatics.GetPlayerCharacter` 0)))
  (set `self.inventario` (`/Game/ThirdPerson/Blueprints/BP_Ingothar.BP_InventoryComponent` _asbp_ingothar))
  (bind _outrownames (`DataTableFunctionLibrary.GetDataTableRowNames` "/Game/xaBoleador/Data_Table/Dt_Shop_aRMADURAS.Dt_Shop_aRMADURAS"))
  (for _array_element _outrownames
    (bind _returnvalue (`|GetDataTableRow` "/Game/xaBoleador/Data_Table/Dt_Shop_aRMADURAS.Dt_Shop_aRMADURAS" _array_element)
      (:`then`
        (`KismetArrayLibrary.Array_Add` (`self.Shop_Armaduras`) _returnvalue))))
  (bind _outrownames_2 (`DataTableFunctionLibrary.GetDataTableRowNames` "/Game/xaBoleador/Data_Table/Dt_shop_Partes_De_Arma.Dt_shop_Partes_De_Arma"))
  (for _array_element_2 _outrownames_2
    (bind _returnvalue_2 (`|GetDataTableRow` "/Game/xaBoleador/Data_Table/Dt_shop_Partes_De_Arma.Dt_shop_Partes_De_Arma" _array_element_2)
      (:`then`
        (`KismetArrayLibrary.Array_Add` (`self.Shop_Partes_Armas`) _returnvalue_2))))
  (bind _outrownames_3 (`DataTableFunctionLibrary.GetDataTableRowNames` "/Game/xaBoleador/Data_Table/Dt_Shop_Materiales.Dt_Shop_Materiales"))
  (for _array_element_3 _outrownames_3
    (bind _returnvalue_3 (`|GetDataTableRow` "/Game/xaBoleador/Data_Table/Dt_Shop_Materiales.Dt_Shop_Materiales" _array_element_3)
      (:`then`
        (`KismetArrayLibrary.Array_Add` (`self.Shop_Materiales`) _returnvalue_3))))
  (bind _outrownames_4 (`DataTableFunctionLibrary.GetDataTableRowNames` "/Game/xaBoleador/Data_Table/DT_Shop_objetosclaves.DT_Shop_objetosclaves"))
  (for _array_element_4 _outrownames_4
    (bind _returnvalue_4 (`|GetDataTableRow` "/Game/xaBoleador/Data_Table/DT_Shop_objetosclaves.DT_Shop_objetosclaves" _array_element_4)
      (:`then`
        (`KismetArrayLibrary.Array_Add` (`self.Shop_Partes_Objetos`) _returnvalue_4)))))

(event `self.Box.OnComponentBeginOverlap`
  (params (OverlappedComponent :type "PrimitiveComponent Object Reference") (OtherActor :type "Actor Object Reference") (OtherComp :type "PrimitiveComponent Object Reference") (OtherBodyIndex :type Integer) (bFromSweep :type Boolean) (SweepResult :type "HitResult Structure (by ref)"))
  (bind _asbp_ingothar (cast `/Game/ThirdPerson/Blueprints/BP_Ingothar` OtherActor))
  (set `/Game/ThirdPerson/Blueprints/BP_Ingothar.Current Tienda` self _asbp_ingothar))

(event `self.Box.OnComponentEndOverlap`
  (params (OverlappedComponent :type "PrimitiveComponent Object Reference") (OtherActor :type "Actor Object Reference") (OtherComp :type "PrimitiveComponent Object Reference") (OtherBodyIndex :type Integer))
  (bind _asbp_ingothar (cast `/Game/ThirdPerson/Blueprints/BP_Ingothar` OtherActor))
  (set `/Game/ThirdPerson/Blueprints/BP_Ingothar.Current Tienda` null _asbp_ingothar))

(event `Repasar lista_p armas`
  (params (`S partes arma` :type "/Game/Krosty/Inventory/Blueprints/S_PartesArmasStruct Structure"))
  (bind (_name _stackable _quantity) (break `/Game/Krosty/Inventory/Blueprints/S_PartesArmasStruct` `S partes arma`))
  (bind _inventario (`self.inventario`))
  (bind _inventario_2 (`self.inventario`))
  (bind _itemspartesarmas (`/Game/Krosty/Blueprints/BP_InventoryComponent.ItemsPartesArmas` (`self.inventario`)))
  (bind _itemspartesarmas_2 (`/Game/Krosty/Blueprints/BP_InventoryComponent.ItemsPartesArmas` (`self.inventario`)))
  (set `self.set item inventario` false)
  (for (_array_element _array_index) _itemspartesarmas_2
    (bind (_name_2 _stackable_2 _quantity_2) (break `/Game/Krosty/Inventory/Blueprints/S_PartesArmasStruct` _array_element))
    (if (`KismetTextLibrary.EqualEqual_TextText` _name_2 _name)
      (if (> (+ _quantity_2 _quantity) 64)
        (break)
        (else
          (bind _output_get (set `self.TEMP INDEX` _array_index))
          (bind (_output_name _output_stackable _output_quantity _output_type _output_thumnail _output_mesh _output_descripciondelitem _output_stats _output_price) (break `/Game/Krosty/Inventory/Blueprints/S_PartesArmasStruct` (`|GetArrayItem` (`/Game/Krosty/Blueprints/BP_InventoryComponent.ItemsPartesArmas` (`self.inventario`)) _output_get)))
          (`KismetArrayLibrary.Array_Set` _itemspartesarmas_2 _array_index (make `/Game/Krosty/Inventory/Blueprints/S_PartesArmasStruct` _output_name _output_stackable (+ _output_quantity _quantity) _output_type _output_thumnail _output_mesh _output_descripciondelitem _output_stats _output_price))
          (set `self.set item inventario` true)
          (`/Game/Krosty/Inventory/Widgets/WB_Inventory.LoadInventoryPartesArmas` (`/Game/Krosty/Blueprints/BP_InventoryComponent.InventoryWidget` _inventario_2) _inventario_2 false (`self.TEMP INDEX`))
          (break)))))
  (if (not (`self.set item inventario`))
    (for (_array_element_2 _array_index_2) _itemspartesarmas :!label _label
      (if (not (> (`.Quantity_13_28028BEF44C31620A0E3EEA07037C568` (break `/Game/Krosty/Inventory/Blueprints/S_PartesArmasStruct` _array_element_2)) 0))
        (set `self.TEMP INDEX` _array_index_2)
        (`KismetArrayLibrary.Array_Set` _itemspartesarmas _array_index_2 `S partes arma`)
        (break)))
    (`/Game/Krosty/Inventory/Widgets/WB_Inventory.LoadInventoryPartesArmas` (`/Game/Krosty/Blueprints/BP_InventoryComponent.InventoryWidget` _inventario) _inventario false (`self.TEMP INDEX`))
    (goto _label :!via `Break`)))

(event `Repasar_lista_Armaduras`
  (params (`Armaduras strucgt` :type "/Game/Krosty/Inventory/Blueprints/S_ArmadurasStruct Structure"))
  (bind (_name _stackable _quantity) (break `/Game/Krosty/Inventory/Blueprints/S_ArmadurasStruct` `Armaduras strucgt`))
  (bind _inventario (`self.inventario`))
  (bind _inventario_2 (`self.inventario`))
  (bind _itemsarmaduras (`/Game/Krosty/Blueprints/BP_InventoryComponent.ItemsArmaduras` (`self.inventario`)))
  (bind _itemsarmaduras_2 (`/Game/Krosty/Blueprints/BP_InventoryComponent.ItemsArmaduras` (`self.inventario`)))
  (set `self.set item inventario` false)
  (for (_array_element _array_index) _itemsarmaduras
    (bind (_name_2 _stackable_2 _quantity_2) (break `/Game/Krosty/Inventory/Blueprints/S_ArmadurasStruct` _array_element))
    (if (`KismetTextLibrary.EqualEqual_TextText` _name _name_2)
      (if (> (+ _quantity_2 _quantity_2) 64)
        (break)
        (else
          (bind _output_get (set `self.TEMP INDEX` _array_index))
          (bind (_output_name _output_stackable _output_quantity _output_thumnail _output_mesh _output_descripciondelitem _output_price _output_stats) (break `/Game/Krosty/Inventory/Blueprints/S_ArmadurasStruct` (`|GetArrayItem` (`/Game/Krosty/Blueprints/BP_InventoryComponent.ItemsArmaduras` (`self.inventario`)) _output_get)))
          (`KismetArrayLibrary.Array_Set` _itemsarmaduras _array_index (make `/Game/Krosty/Inventory/Blueprints/S_ArmadurasStruct` _output_name _output_stackable (+ _output_quantity _quantity) _output_thumnail _output_mesh _output_descripciondelitem _output_price _output_stats))
          (set `self.set item inventario` true)
          (`/Game/Krosty/Inventory/Widgets/WB_Inventory.LoadInventoryArmaduras` (`/Game/Krosty/Blueprints/BP_InventoryComponent.InventoryWidget` _inventario_2) _inventario_2 false (`self.TEMP INDEX`))
          (break)))))
  (if (not (`self.set item inventario`))
    (for (_array_element_2 _array_index_2) _itemsarmaduras_2 :!label _label_2
      (if (not (> (`.Quantity_13_28028BEF44C31620A0E3EEA07037C568` (break `/Game/Krosty/Inventory/Blueprints/S_ArmadurasStruct` _array_element_2)) 0))
        (set `self.TEMP INDEX` _array_index_2)
        (`KismetArrayLibrary.Array_Set` _itemsarmaduras_2 _array_index_2 `Armaduras strucgt`)
        (break)))
    (`/Game/Krosty/Inventory/Widgets/WB_Inventory.LoadInventoryArmaduras` (`/Game/Krosty/Blueprints/BP_InventoryComponent.InventoryWidget` _inventario) _inventario false (`self.TEMP INDEX`))
    (goto _label_2 :!via `Break`)))

(event `Repasarlista_Materiales`
  (params (`s Material shop` :type "/Game/Krosty/Inventory/Blueprints/S_ItemMaterialStruct Structure"))
  (bind (_name _stackable _quantity) (break `/Game/Krosty/Inventory/Blueprints/S_ItemMaterialStruct` `s Material shop`))
  (bind _inventario (`self.inventario`))
  (bind _inventario_2 (`self.inventario`))
  (bind _itemsmateriales (`/Game/Krosty/Blueprints/BP_InventoryComponent.ItemsMateriales` (`self.inventario`)))
  (bind _itemsmateriales_2 (`/Game/Krosty/Blueprints/BP_InventoryComponent.ItemsMateriales` (`self.inventario`)))
  (set `self.set item inventario` false)
  (for (_array_element _array_index) _itemsmateriales
    (bind (_name_2 _stackable_2 _quantity_2) (break `/Game/Krosty/Inventory/Blueprints/S_ItemMaterialStruct` _array_element))
    (if (`KismetTextLibrary.EqualEqual_TextText` _name _name_2)
      (if (> (+ _quantity_2 _quantity_2) 64)
        (break)
        (else
          (bind _output_get (set `self.TEMP INDEX` _array_index))
          (bind (_output_name _output_stackable _output_quantity _output_thumnail _output_mesh _output_descripciondelitem _output_price) (break `/Game/Krosty/Inventory/Blueprints/S_ItemMaterialStruct` (`|GetArrayItem` (`/Game/Krosty/Blueprints/BP_InventoryComponent.ItemsMateriales` (`self.inventario`)) _output_get)))
          (`KismetArrayLibrary.Array_Set` _itemsmateriales _array_index (make `/Game/Krosty/Inventory/Blueprints/S_ItemMaterialStruct` _output_name _output_stackable (+ _output_quantity _quantity) _output_thumnail _output_mesh _output_descripciondelitem _output_price))
          (set `self.set item inventario` true)
          (`/Game/Krosty/Inventory/Widgets/WB_Inventory.LoadInventoryMateriales` (`/Game/Krosty/Blueprints/BP_InventoryComponent.InventoryWidget` _inventario_2) _inventario_2 false (`self.TEMP INDEX`))
          (break)))))
  (if (not (`self.set item inventario`))
    (for (_array_element_2 _array_index_2) _itemsmateriales_2 :!label _label_3
      (if (not (> (`.Quantity_13_28028BEF44C31620A0E3EEA07037C568` (break `/Game/Krosty/Inventory/Blueprints/S_ItemMaterialStruct` _array_element_2)) 0))
        (set `self.TEMP INDEX` _array_index_2)
        (`KismetArrayLibrary.Array_Set` _itemsmateriales_2 _array_index_2 `s Material shop`)
        (break)))
    (`/Game/Krosty/Inventory/Widgets/WB_Inventory.LoadInventoryMateriales` (`/Game/Krosty/Blueprints/BP_InventoryComponent.InventoryWidget` _inventario) _inventario false (`self.TEMP INDEX`))
    (goto _label_3 :!via `Break`)))

(event `Repasar_lista_ObjetosClave`
  (params (`S Objetos Clave` :type "/Game/Krosty/Inventory/Blueprints/S_ObjetosClaveStruct Structure"))
  (bind (_name _stackable _quantity) (break `/Game/Krosty/Inventory/Blueprints/S_ObjetosClaveStruct` `S Objetos Clave`))
  (bind _inventario (`self.inventario`))
  (bind _inventario_2 (`self.inventario`))
  (bind _itemsobjetosclave (`/Game/Krosty/Blueprints/BP_InventoryComponent.ItemsObjetosClave` (`self.inventario`)))
  (bind _itemsobjetosclave_2 (`/Game/Krosty/Blueprints/BP_InventoryComponent.ItemsObjetosClave` (`self.inventario`)))
  (set `self.set item inventario` false)
  (for (_array_element _array_index) _itemsobjetosclave
    (bind (_name_2 _stackable_2 _quantity_2) (break `/Game/Krosty/Inventory/Blueprints/S_ObjetosClaveStruct` _array_element))
    (if (`KismetTextLibrary.EqualEqual_TextText` _name_2 _name)
      (if (> (+ _quantity_2 _quantity_2) 64)
        (break)
        (else
          (bind _output_get (set `self.TEMP INDEX` _array_index))
          (bind (_output_name _output_stackable _output_quantity _output_thumnail _output_mesh _output_descripciondelitem _output_price) (break `/Game/Krosty/Inventory/Blueprints/S_ObjetosClaveStruct` (`|GetArrayItem` (`/Game/Krosty/Blueprints/BP_InventoryComponent.ItemsObjetosClave` (`self.inventario`)) _output_get)))
          (`KismetArrayLibrary.Array_Set` _itemsobjetosclave _array_index (make `/Game/Krosty/Inventory/Blueprints/S_ObjetosClaveStruct` _output_name _output_stackable (+ _output_quantity _quantity) _output_thumnail _output_mesh _output_descripciondelitem _output_price))
          (set `self.set item inventario` true)
          (`/Game/Krosty/Inventory/Widgets/WB_Inventory.LoadInventoryObjetosClave` (`/Game/Krosty/Blueprints/BP_InventoryComponent.InventoryWidget` _inventario_2) _inventario_2 false (`self.TEMP INDEX`))
          (break)))))
  (if (not (`self.set item inventario`))
    (for (_array_element_2 _array_index_2) _itemsobjetosclave_2 :!label _label_4
      (if (not (> (`.Quantity_13_28028BEF44C31620A0E3EEA07037C568` (break `/Game/Krosty/Inventory/Blueprints/S_ObjetosClaveStruct` _array_element_2)) 0))
        (set `self.TEMP INDEX` _array_index_2)
        (`KismetArrayLibrary.Array_Set` _itemsobjetosclave_2 _array_index_2 `S Objetos Clave`)
        (break)))
    (`/Game/Krosty/Inventory/Widgets/WB_Inventory.LoadInventoryObjetosClave` (`/Game/Krosty/Blueprints/BP_InventoryComponent.InventoryWidget` _inventario) _inventario false (`self.TEMP INDEX`))
    (goto _label_4 :!via `Break`)))

(fn `TRYBUY`
  (params (Items :type "/Game/Krosty/Inventory/Blueprints/S_PartesArmasStruct Structure") (`bp tienda` :type "/Game/xaBoleador/Bp/bp_tienda Object Reference") (index :type Integer))
  (returns (`upadete item` :type "/Game/Krosty/Inventory/Blueprints/S_PartesArmasStruct Structure") (CanBuy :type Boolean))
  (bind _s_partesarmasstruct (make `/Game/Krosty/Inventory/Blueprints/S_PartesArmasStruct` Items_NAME_7_2DD24B7040AD4678F4F39A922381E89D Items_Stackable_8_0C99ABDB49B81B32328185999256D245 (- Items_Quantity_13_28028BEF44C31620A0E3EEA07037C568 1) Items_Type_29_C974570B43189C4E446E218BAC153FDC Items_Thumnail_15_D65AB25B4BA1BF3D8E1E178F3B3E18AE Items_Mesh_18_ED2B7F36480B5A06EB21CE9BA7380561 Items_DescripcionDelItem_23_653356574F8BFA6F57569F944A436514 Items_Stats_26_9D32DCF3442601D7B1ECA085D5B5C6A5 Items_Price_32_406AC06949B1AE7F1A29A78FC86D7054))
  (bind _asgame_instance_slice (cast `/Game/GameInstance_Slice` (`GameplayStatics.GetGameInstance`)))
  (bind _gamedata (`/Game/GameInstance_Slice.GameData` _asgame_instance_slice))
  (if (>= (`/Game/xaBoleador/Bp/BP_Save_Games.Currency_Save` _gamedata) Items_Price_32_406AC06949B1AE7F1A29A78FC86D7054)
    (set `/Game/xaBoleador/Bp/BP_Save_Games.Currency_Save` (- (`/Game/xaBoleador/Bp/BP_Save_Games.Currency_Save` _gamedata) Items_Price_32_406AC06949B1AE7F1A29A78FC86D7054) _gamedata)
    (`KismetArrayLibrary.Array_Set` (`self.Shop_Partes_Armas`) index _s_partesarmasstruct)
    (return _s_partesarmasstruct true)
    (else
      (return (struct) false))))

(fn `TryBuy_Armaduras`
  (params (NewParam :type "/Game/Krosty/Inventory/Blueprints/S_ArmadurasStruct Structure") (Index_Item :type Integer))
  (returns (`upadete item` :type "/Game/Krosty/Inventory/Blueprints/S_ArmadurasStruct Structure") (CanBuy :type Boolean))
  (bind _s_armadurasstruct (make `/Game/Krosty/Inventory/Blueprints/S_ArmadurasStruct` NewParam_NAME_7_2DD24B7040AD4678F4F39A922381E89D NewParam_Stackable_8_0C99ABDB49B81B32328185999256D245 (- NewParam_Quantity_13_28028BEF44C31620A0E3EEA07037C568 1) NewParam_Thumnail_15_D65AB25B4BA1BF3D8E1E178F3B3E18AE NewParam_Mesh_18_ED2B7F36480B5A06EB21CE9BA7380561 NewParam_DescripcionDelItem_23_932FC7274DC25D0163F587A0F5F8D1C7 NewParam_Price_26_05B85BA84A135460C8B0E09AD3978B24 NewParam_stats_28_6AA3DD1249CF0861D1A20A9C3A230482))
  (bind _asgame_instance_slice (cast `/Game/GameInstance_Slice` (`GameplayStatics.GetGameInstance`)))
  (bind _gamedata (`/Game/GameInstance_Slice.GameData` _asgame_instance_slice))
  (if (>= (`/Game/xaBoleador/Bp/BP_Save_Games.Currency_Save` _gamedata) NewParam_Price_26_05B85BA84A135460C8B0E09AD3978B24)
    (set `/Game/xaBoleador/Bp/BP_Save_Games.Currency_Save` (- (`/Game/xaBoleador/Bp/BP_Save_Games.Currency_Save` _gamedata) NewParam_Price_26_05B85BA84A135460C8B0E09AD3978B24) _gamedata)
    (`KismetArrayLibrary.Array_Set` (`self.Shop_Armaduras`) Index_Item _s_armadurasstruct)
    (return _s_armadurasstruct true)
    (else
      (return (struct) false))))

(fn `TryBuy_Materiales`
  (params (`S items mat` :type "/Game/Krosty/Inventory/Blueprints/S_ItemMaterialStruct Structure") (`Index Item` :type Integer))
  (returns (`upadete item` :type "/Game/Krosty/Inventory/Blueprints/S_ItemMaterialStruct Structure") (CanBuy :type Boolean))
  (bind _s_itemmaterialstruct (make `/Game/Krosty/Inventory/Blueprints/S_ItemMaterialStruct` `S items mat_NAME_7_2DD24B7040AD4678F4F39A922381E89D` `S items mat_Stackable_8_0C99ABDB49B81B32328185999256D245` (- `S items mat_Quantity_13_28028BEF44C31620A0E3EEA07037C568` 1) `S items mat_Thumnail_15_D65AB25B4BA1BF3D8E1E178F3B3E18AE` `S items mat_Mesh_18_ED2B7F36480B5A06EB21CE9BA7380561` `S items mat_DescripcionDelItem_23_1E613F5E4E6FFEEF8E8CA4A1E6EDED19` `S items mat_Price_26_9C9329AB4992D6255A77378583EE1CD0`))
  (bind _asgame_instance_slice (cast `/Game/GameInstance_Slice` (`GameplayStatics.GetGameInstance`)))
  (bind _gamedata (`/Game/GameInstance_Slice.GameData` _asgame_instance_slice))
  (if (>= (`/Game/xaBoleador/Bp/BP_Save_Games.Currency_Save` _gamedata) `S items mat_Price_26_9C9329AB4992D6255A77378583EE1CD0`)
    (set `/Game/xaBoleador/Bp/BP_Save_Games.Currency_Save` (- (`/Game/xaBoleador/Bp/BP_Save_Games.Currency_Save` _gamedata) `S items mat_Price_26_9C9329AB4992D6255A77378583EE1CD0`) _gamedata)
    (`KismetArrayLibrary.Array_Set` (`self.Shop_Materiales`) `Index Item` _s_itemmaterialstruct)
    (return _s_itemmaterialstruct true)
    (else
      (return (struct) false))))

(fn `TryBuy_Objetos_Claves`
  (params (`S Objetos Claves` :type "/Game/Krosty/Inventory/Blueprints/S_ObjetosClaveStruct Structure") (`Index Item` :type Integer) (BpTienda :type "/Game/xaBoleador/Bp/bp_tienda Object Reference"))
  (returns (`upadete item` :type "/Game/Krosty/Inventory/Blueprints/S_ObjetosClaveStruct Structure") (CanBuy :type Boolean))
  (bind _s_objetosclavestruct (make `/Game/Krosty/Inventory/Blueprints/S_ObjetosClaveStruct` `S Objetos Claves_NAME_7_2DD24B7040AD4678F4F39A922381E89D` `S Objetos Claves_Stackable_8_0C99ABDB49B81B32328185999256D245` (- `S Objetos Claves_Quantity_13_28028BEF44C31620A0E3EEA07037C568` 1) `S Objetos Claves_Thumnail_15_D65AB25B4BA1BF3D8E1E178F3B3E18AE` `S Objetos Claves_Mesh_18_ED2B7F36480B5A06EB21CE9BA7380561` `S Objetos Claves_DescripcionDelItem_23_D68E6C0A49FCEDE6A17D019522FAD975` `S Objetos Claves_Price_26_D115DDE648AB53CAE011C8BA1CD46E4D`))
  (bind _asgame_instance_slice (cast `/Game/GameInstance_Slice` (`GameplayStatics.GetGameInstance`)))
  (bind _gamedata (`/Game/GameInstance_Slice.GameData` _asgame_instance_slice))
  (if (>= (`/Game/xaBoleador/Bp/BP_Save_Games.Currency_Save` _gamedata) `S Objetos Claves_Price_26_D115DDE648AB53CAE011C8BA1CD46E4D`)
    (set `/Game/xaBoleador/Bp/BP_Save_Games.Currency_Save` (- (`/Game/xaBoleador/Bp/BP_Save_Games.Currency_Save` _gamedata) `S Objetos Claves_Price_26_D115DDE648AB53CAE011C8BA1CD46E4D`) _gamedata)
    (`KismetArrayLibrary.Array_Set` (`self.Shop_Partes_Objetos`) `Index Item` _s_objetosclavestruct)
    (return _s_objetosclavestruct true)
    (else
      (return (struct) false))))

(fn `UserConstructionScript`)