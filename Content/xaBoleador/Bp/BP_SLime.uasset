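; Slime enemy that patrols points until pawn sensing or a trigger detects BP_Maria, then chases her.
; In range it randomly plays one of two weighted montages, whose damage triggers subtract player Life; CanAttack is never re-enabled here.
; Sword-tagged overlaps deal fixed damage, causing a movement-locking hit montage or death, which grants EXP and destroys the actor.
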(event `self.ReceiveBeginPlay`
  (bind _asbp_maria (cast `/Game/ThirdPerson/Blueprints/BP_Maria` (`GameplayStatics.GetPlayerPawn` 0)))
  (set `self.PLayer` _asbp_maria)
  (`SkinnedMeshComponent.SetLeaderPoseComponent` (`self.SkeletalMesh1`) (`self.Mesh`) true false))

(event `self.ReceiveTick`
  (params (DeltaSeconds :type "Float (single-precision)"))
  (if (`self.death`)
    _
    (elif (`self.Move to player`)
      (`|AIMoveTo` self (0.0 0.0 0.0) (`self.PLayer`) 10.0
        (:`then`
          (if (<= (`KismetMathLibrary.Vector_Distance` (`self.K2_GetActorLocation` (`self.PLayer`)) (`self.K2_GetActorLocation`)) (`self.Attack Distance`))
            (if (and (`self.Can attack`) (not (`self.is attacking`)))
              (`self.AttackSlime`)))))
      (elif (not (`self.PatrolBool`))
        (`self.Patrol`)))))

(event `Patrol`
  (bind _returnvalue (+ (`self.Patrol Index`) 1))
  ; Patrol
  (if (not (`self.player see`))
    (set `self.PatrolBool` true)
    (`|AIMoveTo` self (`self.K2_GetActorLocation` (`|GetArrayItem` (`self.PatrolsPoints`) (`self.Patrol Index`))) null 200.0 true :!label _label
      (:`OnSuccess`
        (if (>= _returnvalue (`KismetArrayLibrary.Array_Length` (`self.PatrolsPoints`)))
          (set `self.Patrol Index` 0)
          (else
            (set `self.Patrol Index` _returnvalue)))
        (`KismetSystemLibrary.Delay` 1.0)
        (goto _label)))))

(event `self.PawnSensing.OnSeePawn`
  (params (Pawn :type "Pawn Object Reference"))
  ; detecta al player si lo ve
  (cast `/Game/ThirdPerson/Blueprints/BP_Maria` Pawn)
  (if (not (`self.player see`))
    (set `self.player see` true)
    (`MovementComponent.StopMovementImmediately` (`self.CharacterMovement`))
    (bind _asab_anim_slime (cast `/Game/xaBoleador/Enemy/Slime/Anims/AB_Anim_Slime` (`SkeletalMeshComponent.GetAnimInstance` (`self.Mesh`))))
    (set `/Game/xaBoleador/Enemy/Slime/Anims/AB_Anim_Slime.speedSlime` 75.0 _asab_anim_slime)
    (set `self.Move to player` true)))

(event `self.Trigger Detect.OnComponentBeginOverlap`
  (params (OverlappedComponent :type "PrimitiveComponent Object Reference") (OtherActor :type "Actor Object Reference") (OtherComp :type "PrimitiveComponent Object Reference") (OtherBodyIndex :type Integer) (bFromSweep :type Boolean) (SweepResult :type "HitResult Structure (by ref)"))
  ; Detecta trigger y va a x ti
  (cast `/Game/ThirdPerson/Blueprints/BP_Maria` OtherActor)
  (if (not (`self.player see`))
    (set `self.player see` true)
    (`MovementComponent.StopMovementImmediately` (`self.CharacterMovement`))
    (bind _asab_anim_slime (cast `/Game/xaBoleador/Enemy/Slime/Anims/AB_Anim_Slime` (`SkeletalMeshComponent.GetAnimInstance` (`self.Mesh`))))
    (set `/Game/xaBoleador/Enemy/Slime/Anims/AB_Anim_Slime.speedSlime` 75.0 _asab_anim_slime)
    (set `self.Move to player` true)))

(event `AttackSlime`
  ; Ataques
  (set `self.is attacking` true)
  (set `self.Move to player` false)
  (if (`self.Can attack`)
    (set `self.Can attack` false)
    (set `self.Cooldown` true)
    (`MovementComponent.StopMovementImmediately` (`self.CharacterMovement`))
    (if (`KismetMathLibrary.RandomBoolWithWeight` 0.7)
      (bind _returnvalue (`self.PlayAnimMontage` "/Game/xaBoleador/Enemy/Slime/Anims/Slime_Attack_basic.Slime_Attack_basic"))
      (`KismetSystemLibrary.Delay` _returnvalue)
      (set `self.is attacking` false)
      (set `self.Move to player` true)
      (else
        (bind _returnvalue_2 (`self.PlayAnimMontage` "/Game/xaBoleador/Enemy/Slime/Anims/Slime_Attack_2.Slime_Attack_2"))
        (`KismetSystemLibrary.Delay` _returnvalue_2)
        (set `self.is attacking` false)
        (set `self.Move to player` true)))))

(event `self.Trigger Detect.OnComponentEndOverlap`
  (params (OverlappedComponent :type "PrimitiveComponent Object Reference") (OtherActor :type "Actor Object Reference") (OtherComp :type "PrimitiveComponent Object Reference") (OtherBodyIndex :type Integer))
  (cast `/Game/ThirdPerson/Blueprints/BP_Maria` OtherActor)
  (set `self.Move to player` false)
  (set `self.player see` false))

(event `self.DamageTriggerattack1.OnComponentBeginOverlap`
  (params (OverlappedComponent :type "PrimitiveComponent Object Reference") (OtherActor :type "Actor Object Reference") (OtherComp :type "PrimitiveComponent Object Reference") (OtherBodyIndex :type Integer) (bFromSweep :type Boolean) (SweepResult :type "HitResult Structure (by ref)"))
  (if (`self.is attacking`)
    (bind _asbp_maria (cast `/Game/ThirdPerson/Blueprints/BP_Maria` OtherActor))
    (bind _statuscomponent (`/Game/ThirdPerson/Blueprints/BP_Maria.StatusComponent` _asbp_maria))
    (set `/Game/Krosty/Blueprints/StatusComponent.life` (- (`/Game/Krosty/Blueprints/StatusComponent.life` _statuscomponent) (`self.damage enemy_Attack1`)) _statuscomponent)
    (`KismetSystemLibrary.PrintString` "1")))

(event `self.DamageTriggerattack2.OnComponentBeginOverlap`
  (params (OverlappedComponent :type "PrimitiveComponent Object Reference") (OtherActor :type "Actor Object Reference") (OtherComp :type "PrimitiveComponent Object Reference") (OtherBodyIndex :type Integer) (bFromSweep :type Boolean) (SweepResult :type "HitResult Structure (by ref)"))
  (`KismetSystemLibrary.PrintString` (`KismetSystemLibrary.GetDisplayName` OtherActor))
  (if (`self.is attacking`)
    (bind _asbp_maria (cast `/Game/ThirdPerson/Blueprints/BP_Maria` OtherActor))
    (bind _statuscomponent (`/Game/ThirdPerson/Blueprints/BP_Maria.StatusComponent` _asbp_maria))
    (set `/Game/Krosty/Blueprints/StatusComponent.life` (- (`/Game/Krosty/Blueprints/StatusComponent.life` _statuscomponent) (`self.damage enemy_attack2`)) _statuscomponent)
    (`KismetSystemLibrary.PrintString` "2")))

(event `TakeDamage`
  (params (DamageSword :type "Float (double-precision)" :default 30.0))
  (bind _charactermovement (`self.CharacterMovement`))
  (bind _returnvalue (- (`self.Vida`) DamageSword))
  ; Take Dmg
  (if (<= _returnvalue 0.0)
    (set `self.death` true)
    (bind _asgame_instance_slice (cast `/Game/GameInstance_Slice` (`GameplayStatics.GetGameInstance`)))
    (set `/Game/GameInstance_Slice.EXP_Pj` (+ (`/Game/GameInstance_Slice.EXP_Pj` _asgame_instance_slice) 20.0) _asgame_instance_slice)
    (`KismetSystemLibrary.PrintString` "Montage de muerte")
    (`KismetSystemLibrary.Delay` 2.0)
    (`self.K2_DestroyActor`)
    (else
      (`KismetSystemLibrary.PrintString` "hit animation")
      (set `self.Hit` true)
      (`|PlayMontage` null "/Game/xaBoleador/Enemy/Slime/Anims/Slime_Hit.Slime_Hit"
        (:`then`
          (`CharacterMovementComponent.DisableMovement` _charactermovement)
          (set `self.Vida` _returnvalue))
        (:`OnCompleted`
          (set `self.Hit` false)
          (`CharacterMovementComponent.SetMovementMode` _charactermovement "MOVE_Walking" 0))))))

(event `self.CapsuleComponent.OnComponentBeginOverlap`
  (params (OverlappedComponent :type "PrimitiveComponent Object Reference") (OtherActor :type "Actor Object Reference") (OtherComp :type "PrimitiveComponent Object Reference") (OtherBodyIndex :type Integer) (bFromSweep :type Boolean) (SweepResult :type "HitResult Structure (by ref)"))
  ; Take Dmg
  (if (== "Sword" (`|GetArrayItem` (`ActorComponent.ComponentTags` OtherComp)))
    (`self.TakeDamage` 30.0)))

(fn `TryAttack`
  (if (`self.Attack in range`)
    (if (`self.Can attack`)
      (`self.AttackSlime`))))

(fn `UserConstructionScript`)