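; Bonfire checkpoint actor (hoguera) with a flag that changes from a "bad" to a "good" version once unlocked.
; When BP_Ingothar enters the box, it saves its spawn point as last checkpoint and marks its HogueraInt index unlocked in GameInstance_Slice's GameData.
; BeginPlay reads that flag and, if set, runs CambioMesh, using chained timelines and dynamic materials to dissolve between flag meshes.
; Overlap itself never triggers the swap.
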(event `self.ReceiveTick`
  (params (DeltaSeconds :type "Float (single-precision)"))
  (set `self.Delta Seconds` DeltaSeconds))

(event `self.ReceiveBeginPlay`
  (bind _hogueraint (`self.hogueraInt`))
  (`|ExecutionSequence`
    (:`then_0`
      (`KismetSystemLibrary.Delay` 0.2)
      (set `self.Spawn` (`SceneComponent.K2_GetComponentToWorld` (`self.spawnhoguersa`)))
      (bind _asgame_instance_slice (cast `/Game/GameInstance_Slice` (`GameplayStatics.GetGameInstance`)))
      (`/Engine/EditorBlueprintResources/StandardMacros.IsValid` (`/Game/GameInstance_Slice.GameData` _asgame_instance_slice)
        (:`Is Valid`
          (set `self.Namehoguera` (`|GetArrayItem` (`/Game/GameInstance_Slice.NameHogueras` _asgame_instance_slice) (`self.hogueraInt`))))))
    (:`then_1`
      (bind _returnvalue (`PrimitiveComponent.CreateDynamicMaterialInstance` (`self.StaticMesh`) 0 "/Game/Dani/materials/Flag/MI_Flag_MALA.MI_Flag_MALA" "None"))
      (set `self.MMaterial bandera mala` _returnvalue))
    (:`then_2`
      (bind _asgame_instance_slice_2 (cast `/Game/GameInstance_Slice` (`GameplayStatics.GetGameInstance`)))
      (bind _hogueras_bools_save (`/Game/xaBoleador/Bp/BP_Save_Games.Hogueras_Bools_save` (`/Game/GameInstance_Slice.GameData` _asgame_instance_slice_2)))
      (if (> (`KismetArrayLibrary.Array_Length` _hogueras_bools_save) _hogueraint)
        (if (`|GetArrayItem` _hogueras_bools_save _hogueraint)
          (`self.Cambio Mesh`))))))

(event `self.Box.OnComponentBeginOverlap`
  (params (OverlappedComponent :type "PrimitiveComponent Object Reference") (OtherActor :type "Actor Object Reference") (OtherComp :type "PrimitiveComponent Object Reference") (OtherBodyIndex :type Integer) (bFromSweep :type Boolean) (SweepResult :type "HitResult Structure (by ref)"))
  (bind _spawn_location (`KismetMathLibrary.BreakTransform` (`self.Spawn`)))
  (cast `/Game/ThirdPerson/Blueprints/BP_Ingothar` OtherActor)
  (set `self.PlayerDentro` true)
  (bind _asgame_instance_slice (cast `/Game/GameInstance_Slice` (`GameplayStatics.GetGameInstance`)))
  (bind _gamedata (`/Game/GameInstance_Slice.GameData` _asgame_instance_slice))
  (set `/Game/xaBoleador/Bp/BP_Save_Games.LastCheckpoint_save` _spawn_location _gamedata)
  (set `/Game/xaBoleador/Bp/BP_Save_Games.Hoguera_Actual_save` null _gamedata)
  (if (not (`|GetArrayItem` (`/Game/xaBoleador/Bp/BP_Save_Games.Hogueras_Bools_save` _gamedata) (`self.hogueraInt`)))
    (`KismetArrayLibrary.Array_Set` (`/Game/xaBoleador/Bp/BP_Save_Games.Hogueras_Bools_save` (`/Game/GameInstance_Slice.GameData` _asgame_instance_slice)) (`self.hogueraInt`) true)))

(event `MenuOpen`)

(event `self.Box.OnComponentEndOverlap`
  (params (OverlappedComponent :type "PrimitiveComponent Object Reference") (OtherActor :type "Actor Object Reference") (OtherComp :type "PrimitiveComponent Object Reference") (OtherBodyIndex :type Integer))
  (cast `/Game/ThirdPerson/Blueprints/BP_Ingothar` OtherActor)
  (set `self.PlayerDentro` false))

(event `Cambio Mesh`
  (if (not (`self.primera vez`))
    (cast `/Game/GameInstance_Slice` (`GameplayStatics.GetGameInstance`))
    (bind (_direction _dissolvevalue) (`Timeline|timeline` :!via `PlayFromStart`)
      (:`Update`
        (`MaterialInstanceDynamic.SetScalarParameterValue` (`self.MMaterial bandera mala`) "Dissolve" _dissolvevalue))
      (:`Finished`
        (bind _returnvalue (`PrimitiveComponent.CreateDynamicMaterialInstance` (`self.StaticMesh`) 0 "/Game/Dani/materials/Flag/MI_Flag_BUENA.MI_Flag_BUENA" "None"))
        (set `self.material bandera buena` _returnvalue)
        (`StaticMeshComponent.SetStaticMesh` (`self.StaticMesh`) "/Game/Dani/meshes/hogueras/BANDERA_BUENA.BANDERA_BUENA")
        (bind (_direction_2 _dissolvevalue_2) (`Timeline|Timeline` :!via `PlayFromStart`)
          (:`Update`
            (`MaterialInstanceDynamic.SetScalarParameterValue` (`self.material bandera buena`) "Dissolve" _dissolvevalue_2)
            (set `self.primera vez` true)))))))

(fn `UserConstructionScript`)