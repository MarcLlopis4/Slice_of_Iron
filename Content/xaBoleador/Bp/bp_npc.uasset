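; NPC actor that runs branching, data-table-driven dialogue with the player.
; Its box registers it on BP_Maria; Interact opens Ui_Dialogue or advances it, each row supplying the next row, table and end flag.
; ShowButtons lists the opening row's choices as UI_Options_Dialogue widgets, while Options_Respuesta loads a given row and its choices.
; Ending the dialogue or leaving the box removes the UI, restores game input and, after a delay, blends the camera to the player.
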(event `/Game/xaBoleador/Bp/bp_ui_npc.LeaveDialogue`
  (bind _returnvalue (`GameplayStatics.GetPlayerController` 0))
  (`/Engine/EditorBlueprintResources/StandardMacros.IsValid` (`self.UiWidget`)
    (:`Is Valid`
      (`Widget.RemoveFromParent` (`self.UiWidget`))
      (`Widget.RemoveFromParent` (`self.UiWidget`) :!label _label)
      (set `self.EndDialogue` false)
      (set `self.UiWidget` null)
      (`WidgetBlueprintLibrary.SetInputMode_GameOnly` _returnvalue)
      (set `PlayerController.bShowMouseCursor` false _returnvalue)
      (`KismetSystemLibrary.Delay` 1.0)
      (`PlayerController.SetViewTargetWithBlend` (`GameplayStatics.GetPlayerController` 0) (`GameplayStatics.GetPlayerCharacter` 0) 0.0 "VTBlend_EaseInOut" 0.0 false))))

(event `Options_Respuesta`
  (params (RowName :type Name) (DataTable :type "DataTable Object Reference"))
  (bind _uiwidget (`self.UiWidget`))
  (bind _returnvalue (`|GetDataTableRow` DataTable RowName)
    (:`then`
      (`PanelWidget.ClearChildren` (`/Game/xaBoleador/Ui/Npc/ui_Dialogue.OptionsScroll` _uiwidget))
      (bind (_dialogue _row _datatable _enddialogue _opendialogue _openoptionsdialogue) (break `/Game/xaBoleador/Structs_No_armas/Dialogue_npc` _returnvalue))
      (`/Game/xaBoleador/Ui/Npc/ui_Dialogue.update dialogue` _uiwidget _dialogue self)
      (set `self.RowName` _row)
      (set `self.Data Table` _datatable)
      (set `self.EndDialogue` _enddialogue)
      (if _opendialogue
        (for _array_element _openoptionsdialogue
          (bind (_option_name _row_2 _datatalbe) (break `/Game/xaBoleador/Structs_No_armas/Respuestas_Dialogue` _array_element))
          (bind _returnvalue_2 (`|CreateWidget` "/Game/xaBoleador/Ui/Npc/UI_Options_Dialogue.UI_Options_Dialogue_C" null (`KismetTextLibrary.Conv_NameToText` _option_name) self _row_2 _datatalbe))
          (`PanelWidget.AddChild` (`/Game/xaBoleador/Ui/Npc/ui_Dialogue.OptionsScroll` (`self.UiWidget`)) _returnvalue_2))))))

(event `/Game/xaBoleador/Bp/bp_ui_npc.Interact`
  (params (player :type "/Game/ThirdPerson/Blueprints/BP_Maria Object Reference"))
  (bind _returnvalue (`GameplayStatics.GetPlayerController` 0))
  (if (`self.EndDialogue`)
    (set `self.IsDialogue` true)
    (goto _label)
    (else
      (set `self.IsDialogue` true)
      (`/Engine/EditorBlueprintResources/StandardMacros.IsValid` (`self.UiWidget`)
        (:`Is Valid`
          (`KismetSystemLibrary.PrintString` "is valid")
          (bind _returnvalue_2 (`|GetDataTableRow` (`self.Data Table`) (`self.RowName`))
            (:`then`
              (bind (_dialogue _row _datatable _enddialogue) (break `/Game/xaBoleador/Structs_No_armas/Dialogue_npc` _returnvalue_2))
              (`/Game/xaBoleador/Ui/Npc/ui_Dialogue.update dialogue` (`self.UiWidget`) _dialogue self)
              (set `self.RowName` _row)
              (set `self.Data Table` _datatable)
              (set `self.EndDialogue` _enddialogue))))
        (:`Is Not Valid`
          (bind _returnvalue_3 (`|GetDataTableRow` (`self.Data Table`) (`self.RowName`))
            (:`then`
              (set `self.DialogoActual` _returnvalue_3)
              (bind (_dialogue_2 _row_2 _datatable_2 _enddialogue_2 _opendialogue _openoptionsdialogue) (break `/Game/xaBoleador/Structs_No_armas/Dialogue_npc` _returnvalue_3))
              (bind _returnvalue_4 (`|CreateWidget` "/Game/xaBoleador/Ui/Npc/ui_Dialogue.ui_Dialogue_C" (`GameplayStatics.GetPlayerController` 0) (`KismetTextLibrary.Conv_NameToText` (`self.Name`)) (`KismetTextLibrary.Conv_TextToString` _dialogue_2) self))
              (bind _output_get (set `self.UiWidget` _returnvalue_4))
              (`UserWidget.AddToViewport` _output_get 0)
              (set `self.RowName` _row_2)
              (set `self.Data Table` _datatable_2)
              (set `self.EndDialogue` _enddialogue_2)
              (`WidgetBlueprintLibrary.SetInputMode_GameAndUIEx` _returnvalue null)
              (set `PlayerController.bShowMouseCursor` true _returnvalue)
              (if _opendialogue
                _))))))))

(event `ShowButtons`
  (for _array_element (`.OpenOptionsDialogue_22_C283D10F40C98AB0BEA8B88C6918895B` (break `/Game/xaBoleador/Structs_No_armas/Dialogue_npc` (`self.DialogoActual`)))
    (bind (_option_name _row _datatalbe) (break `/Game/xaBoleador/Structs_No_armas/Respuestas_Dialogue` _array_element))
    (bind _returnvalue (`|CreateWidget` "/Game/xaBoleador/Ui/Npc/UI_Options_Dialogue.UI_Options_Dialogue_C" null (`KismetTextLibrary.Conv_NameToText` _option_name) self _row _datatalbe))
    (`PanelWidget.AddChild` (`/Game/xaBoleador/Ui/Npc/ui_Dialogue.OptionsScroll` (`self.UiWidget`)) _returnvalue)))

(event `self.Box.OnComponentBeginOverlap`
  (params (OverlappedComponent :type "PrimitiveComponent Object Reference") (OtherActor :type "Actor Object Reference") (OtherComp :type "PrimitiveComponent Object Reference") (OtherBodyIndex :type Integer) (bFromSweep :type Boolean) (SweepResult :type "HitResult Structure (by ref)"))
  (bind _asbp_maria (cast `/Game/ThirdPerson/Blueprints/BP_Maria` OtherActor))
  (set `/Game/ThirdPerson/Blueprints/BP_Maria.NPC` self _asbp_maria))

(event `self.Box.OnComponentEndOverlap`
  (params (OverlappedComponent :type "PrimitiveComponent Object Reference") (OtherActor :type "Actor Object Reference") (OtherComp :type "PrimitiveComponent Object Reference") (OtherBodyIndex :type Integer))
  (bind _asbp_maria (cast `/Game/ThirdPerson/Blueprints/BP_Maria` OtherActor))
  (`self.LeaveDialogue`)
  (set `/Game/ThirdPerson/Blueprints/BP_Maria.NPC` null _asbp_maria))

(fn `UserConstructionScript`)