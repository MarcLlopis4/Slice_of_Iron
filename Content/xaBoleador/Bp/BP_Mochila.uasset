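; BP_Mochila is a backpack Blueprint that handles potion consumption.
; Its UsarPotis event casts the game instance to GameInstance_Slice and, while the Pociones count is above zero, decrements it by one.
; The event applies no potion effect; an unconnected node that would zero the saved potion count never runs.
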(event `Usar Potis`
  (bind _asgame_instance_slice (cast `/Game/GameInstance_Slice` (`GameplayStatics.GetGameInstance`)))
  (if (> (`/Game/GameInstance_Slice.Pociones` _asgame_instance_slice) 0)
    (set `/Game/GameInstance_Slice.Pociones` (- (`/Game/GameInstance_Slice.Pociones` _asgame_instance_slice) 1) _asgame_instance_slice)))

(fn `UserConstructionScript`)