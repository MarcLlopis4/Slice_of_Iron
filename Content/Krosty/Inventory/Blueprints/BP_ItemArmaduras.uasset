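; BP_ItemArmaduras is an armor item actor, apparently a world drop, with a physics-simulated mesh and a tier-based visual effect.
; The construction script sets the static mesh from the InfoItemArmaduras data and turns on physics simulation.
; On BeginPlay, a switch on Tier assigns one of five drop-level Niagara systems to the Niagara component.
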(event `self.ReceiveBeginPlay`
  (switch `int` (`self.Tier`)
    (:`1`
      (`NiagaraComponent.SetAsset` (`self.Niagara`) "/Game/Adri/Niagara/ItemDrop/NS_Droplvl1.NS_Droplvl1" true))
    (:`2`
      (`NiagaraComponent.SetAsset` (`self.Niagara`) "/Game/Adri/Niagara/ItemDrop/NS_Droplvl2.NS_Droplvl2" true))
    (:`3`
      (`NiagaraComponent.SetAsset` (`self.Niagara`) "/Game/Adri/Niagara/ItemDrop/NS_Droplvl3.NS_Droplvl3" true))
    (:`4`
      (`NiagaraComponent.SetAsset` (`self.Niagara`) "/Game/Adri/Niagara/ItemDrop/NS_Droplvl4.NS_Droplvl4" true))
    (:`5`
      (`NiagaraComponent.SetAsset` (`self.Niagara`) "/Game/Adri/Niagara/ItemDrop/NS_Droplvl5.NS_Droplvl5" true))))

(fn `UserConstructionScript`
  (bind _staticmesh (`self.StaticMesh`))
  (`StaticMeshComponent.SetStaticMesh` _staticmesh (`.Mesh_18_ED2B7F36480B5A06EB21CE9BA7380561` (break `/Game/Krosty/Inventory/Blueprints/S_ArmadurasStruct` (`self.InfoItemArmaduras`))))
  (`PrimitiveComponent.SetSimulatePhysics` _staticmesh true))