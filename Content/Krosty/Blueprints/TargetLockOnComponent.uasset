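; Target lock-on component that keeps BP_Maria's camera on a nearby enemy.
; A sphere trace gathers "Enemy"-tagged actors, and line traces plus camera-forward dot products pick the most centred one.
; A looping timer interpolates control rotation toward a distance-lowered aim point while look input is ignored, stopping beyond range or when IsLock is set.
; Left/right switching chooses another centred target by the hit normal's sign against camera right.
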(event `self.ReceiveBeginPlay`
  ; Begin Play - Set player reference
  (set `self.PlayerRef` (cast `/Game/ThirdPerson/Blueprints/BP_Maria` (`GameplayStatics.GetPlayerCharacter` 0) :!pure true)))

(event `Stop Target Lock On`
  (`KismetSystemLibrary.K2_ClearAndInvalidateTimerHandle` (stale `Trigger Target Lock On` _returnvalue))
  (`Controller.ResetIgnoreLookInput` (`GameplayStatics.GetPlayerController` 0)))

(event `Trigger Target Lock On`
  (bind _targetstolockon (`self.CheckForClosestTargets` (`self.TraceForTargets`)))
  (`/Engine/EditorBlueprintResources/StandardMacros.IsValid` _targetstolockon
    (:`Is Valid`
      (set `self.TargetLockedOn` _targetstolockon)
      (`Controller.SetIgnoreLookInput` (`GameplayStatics.GetPlayerController` 0) true)
      (bind _returnvalue (`KismetSystemLibrary.K2_SetTimerDelegate` (delegate `TargetLockOn`) (`GameplayStatics.GetWorldDeltaSeconds`) true)))))

(event `TargetLockOn`
  (bind _returnvalue (`Pawn.GetController` (`self.PlayerRef`)))
  (bind _returnvalue_2 (`Controller.GetControlRotation` _returnvalue))
  (bind (_returnvalue_roll _returnvalue_pitch _returnvalue_yaw) (`KismetMathLibrary.BreakRotator` (`KismetMathLibrary.RInterpTo` _returnvalue_2 (`self.GetLockOnCameraRotation`) 0.01 10.0)))
  (if (or (> (`KismetMathLibrary.Vector_Distance` (`Actor.K2_GetActorLocation` (`self.PlayerRef`)) (`Actor.K2_GetActorLocation` (`self.TargetLockedOn`))) (`self.LockOnRadius`)) (`self.IsLock`))
    (`self.Stop Target Lock On`)
    (else
      (`Controller.SetControlRotation` _returnvalue (`KismetMathLibrary.MakeRotator` (.roll _returnvalue_2) _returnvalue_pitch _returnvalue_yaw)))))

(event `Switch Target On Left`
  (`/Engine/EditorBlueprintResources/StandardMacros.IsValid` (`self.TargetLockedOn`)
    (:`Is Valid`
      (bind _lefttarget (`self.Get Target On Left`))
      (`/Engine/EditorBlueprintResources/StandardMacros.IsValid` _lefttarget
        (:`Is Valid`
          (set `self.TargetLockedOn` _lefttarget))))))

(event `Switch Target on Right`
  (`/Engine/EditorBlueprintResources/StandardMacros.IsValid` (`self.TargetLockedOn`)
    (:`Is Valid`
      (bind _lefttarget (`self.Get Target On Right`))
      (`/Engine/EditorBlueprintResources/StandardMacros.IsValid` _lefttarget
        (:`Is Valid`
          (set `self.TargetLockedOn` _lefttarget))))))

(fn `Check how Close Target Is to Center`
  (params (Target :type "Actor Object Reference"))
  (returns (ReturnValue :type "Float (double-precision)"))
  (bind _playerref (`self.PlayerRef`))
  (return (`KismetMathLibrary.Dot_VectorVector` (`SceneComponent.GetForwardVector` (`/Game/ThirdPerson/Blueprints/BP_Maria.FollowCamera` _playerref)) (`KismetMathLibrary.Conv_RotatorToVector` (`KismetMathLibrary.FindLookAtRotation` (`Actor.K2_GetActorLocation` _playerref) (`Actor.K2_GetActorLocation` Target))))))

(fn `CheckForClosestTargets`
  (params (Targets :type "Array of Actor Object Reference"))
  (returns (TargetsToLockOn :type "Actor Object Reference"))
  (locals (LocalCompareFloat :type "Float (double-precision)") (LocalTargetToLocockOn :type "Actor Object Reference"))
  (for _array_element Targets
    (bind (_outhit _returnvalue) (`KismetSystemLibrary.LineTraceSingle` :`Start` (`SceneComponent.K2_GetComponentLocation` (`/Game/ThirdPerson/Blueprints/BP_Maria.FollowCamera` (`self.PlayerRef`))) :`End` (`Actor.K2_GetActorLocation` _array_element) :`TraceChannel` "TraceTypeQuery1" :`DrawDebugType` "ForDuration"))
    (if _returnvalue
      (bind _returnvalue_2 (`self.Check how Close Target Is to Center` _array_element))
      (`/Engine/EditorBlueprintResources/StandardMacros.CompareFloat` _returnvalue_2 (`local.LocalCompareFloat`)
        (:`>`
          (set `local.LocalCompareFloat` _returnvalue_2)
          (set `local.LocalTargetToLocockOn` _array_element)))))
  (return (`local.LocalTargetToLocockOn`)))

(fn `Get Target On Left`
  (returns (LeftTarget :type "Actor Object Reference"))
  (locals (TargetCompareFloat :type "Float (double-precision)") (TargetToLockOn :type "Actor Object Reference"))
  (for _array_element (`self.TraceForTargets`)
    (bind (_outhit _returnvalue) (`KismetSystemLibrary.LineTraceSingleForObjects` (`SceneComponent.K2_GetComponentLocation` (`/Game/ThirdPerson/Blueprints/BP_Maria.FollowCamera` (`self.PlayerRef`))) (`Actor.K2_GetActorLocation` _array_element) (`|MakeArray` "ObjectTypeQuery7" :!type "EObjectTypeQuery Enum")))
    (if _returnvalue
      (if (and (!= (`self.TargetLockedOn`) _array_element) (> (`KismetMathLibrary.DegAsin` (`KismetMathLibrary.Dot_VectorVector` (`SceneComponent.GetRightVector` (`/Game/ThirdPerson/Blueprints/BP_Maria.FollowCamera` (`self.PlayerRef`))) (`.Normal` (`GameplayStatics.BreakHitResult` _outhit)))) 0.0))
        (bind _returnvalue_2 (`self.Check how Close Target Is to Center` _array_element))
        (`/Engine/EditorBlueprintResources/StandardMacros.CompareFloat` _returnvalue_2 (`local.TargetCompareFloat`)
          (:`>`
            (set `local.TargetCompareFloat` _returnvalue_2)
            (set `local.TargetToLockOn` _array_element))))))
  (return (`local.TargetToLockOn`)))

(fn `Get Target On Right`
  (returns (LeftTarget :type "Actor Object Reference"))
  (locals (TargetCompareFloat :type "Float (double-precision)") (TargetToLockOn :type "Actor Object Reference"))
  (for _array_element (`self.TraceForTargets`)
    (bind (_outhit _returnvalue) (`KismetSystemLibrary.LineTraceSingleForObjects` (`SceneComponent.K2_GetComponentLocation` (`/Game/ThirdPerson/Blueprints/BP_Maria.FollowCamera` (`self.PlayerRef`))) (`Actor.K2_GetActorLocation` _array_element) (`|MakeArray` "ObjectTypeQuery7" :!type "EObjectTypeQuery Enum")))
    (if _returnvalue
      (if (and (!= (`self.TargetLockedOn`) _array_element) (< (`KismetMathLibrary.DegAsin` (`KismetMathLibrary.Dot_VectorVector` (`SceneComponent.GetRightVector` (`/Game/ThirdPerson/Blueprints/BP_Maria.FollowCamera` (`self.PlayerRef`))) (`.Normal` (`GameplayStatics.BreakHitResult` _outhit)))) 0.0))
        (bind _returnvalue_2 (`self.Check how Close Target Is to Center` _array_element))
        (`/Engine/EditorBlueprintResources/StandardMacros.CompareFloat` _returnvalue_2 (`local.TargetCompareFloat`)
          (:`>`
            (set `local.TargetCompareFloat` _returnvalue_2)
            (set `local.TargetToLockOn` _array_element))))))
  (return (`local.TargetToLockOn`)))

(fn `GetLockOnCameraRotation`
  (returns (ReturnValue :type "Rotator Structure"))
  (bind (_returnvalue_x _returnvalue_y _returnvalue_z) (`KismetMathLibrary.BreakVector` (`Actor.K2_GetActorLocation` (`self.TargetLockedOn`))))
  (return (`KismetMathLibrary.FindLookAtRotation` (`SceneComponent.K2_GetComponentLocation` (`/Game/ThirdPerson/Blueprints/BP_Maria.FollowCamera` (`self.PlayerRef`))) (`KismetMathLibrary.MakeVector` _returnvalue_x _returnvalue_y (- _returnvalue_z (/ (`KismetMathLibrary.Vector_Distance` (`Actor.K2_GetActorLocation` (`self.PlayerRef`)) (`Actor.K2_GetActorLocation` (`self.TargetLockedOn`))) 2.0))))))

(fn `TraceForTargets`
  (returns (Targets :type "Array of Actor Object Reference"))
  (locals (LocalTargets :type "Array of Actor Object Reference"))
  (bind _returnvalue (`Actor.K2_GetActorLocation` (`self.PlayerRef`)))
  (bind (_outhits _returnvalue_2) (`KismetSystemLibrary.SphereTraceMultiForObjects` :`Start` _returnvalue :`End` _returnvalue :`Radius` (`self.LockOnRadius`) :`ObjectTypes` (`|MakeArray` "ObjectTypeQuery7" :!type "EObjectTypeQuery Enum") :`DrawDebugType` "ForDuration"))
  (if _returnvalue_2
    (for _array_element _outhits
      (bind (_bblockinghit _binitialoverlap _time _distance _location _impactpoint _normal _impactnormal _physmat _hitactor) (`GameplayStatics.BreakHitResult` _array_element))
      (if (== (`|GetArrayItem` (`Actor.Tags` _hitactor)) "Enemy")
        (`KismetArrayLibrary.Array_Add` (`local.LocalTargets`) _hitactor)))
    (return (`local.LocalTargets`))))