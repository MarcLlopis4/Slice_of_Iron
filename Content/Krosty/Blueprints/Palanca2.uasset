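; Lever actor (Palanca2) that rotates down when BajarPalanca is called, then plays its raising animation after a delay.
; Its Box overlap registers and clears the lever on the BP_Ingothar character's InfoPalanca2 and toggles EstoyDentro.
; Two timelines drive the mesh's rotation lerp.
; The Delay leading to SubidaDePilon hangs off BajadaAlPilon's Update, so its countdown starts as lowering begins.
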(event `self.Box.OnComponentBeginOverlap`
  (params (OverlappedComponent :type "PrimitiveComponent Object Reference") (OtherActor :type "Actor Object Reference") (OtherComp :type "PrimitiveComponent Object Reference") (OtherBodyIndex :type Integer) (bFromSweep :type Boolean) (SweepResult :type "HitResult Structure (by ref)"))
  (bind _asbp_ingothar (cast `/Game/ThirdPerson/Blueprints/BP_Ingothar` OtherActor))
  (set `/Game/ThirdPerson/Blueprints/BP_Ingothar.infoPalanca_2` self _asbp_ingothar)
  (set `self.EstoyDentro` true))

(event `self.Box.OnComponentEndOverlap`
  (params (OverlappedComponent :type "PrimitiveComponent Object Reference") (OtherActor :type "Actor Object Reference") (OtherComp :type "PrimitiveComponent Object Reference") (OtherBodyIndex :type Integer))
  (bind _asbp_ingothar (cast `/Game/ThirdPerson/Blueprints/BP_Ingothar` OtherActor))
  (set `/Game/ThirdPerson/Blueprints/BP_Ingothar.infoPalanca_2` null _asbp_ingothar)
  (set `self.EstoyDentro` false))

(event `BajarPalanca`
  (bind (_direction _newtrack_0) (`Timeline|BajadaAlPilon` :!via `PlayFromStart`)
    (:`Update`
      (`SceneComponent.K2_SetRelativeRotation` (`self.Palanca2`) (`KismetMathLibrary.RLerp` (struct :`Yaw` -90.0) (struct :`Pitch` 55.0 :`Yaw` -90.0) _newtrack_0 true) false false)
      (`KismetSystemLibrary.Delay` 5.0)
      (bind (_direction_2 _newtrack_0_2) (`Timeline|SubidaDePilon` :!via `PlayFromStart`)
        (:`Update`
          (`SceneComponent.K2_SetRelativeRotation` (`self.Palanca2`) (`KismetMathLibrary.RLerp` (struct :`Yaw` -90.0) (struct :`Pitch` 55.0 :`Yaw` -90.0) _newtrack_0_2 true) false false))))))

(fn `UserConstructionScript`)