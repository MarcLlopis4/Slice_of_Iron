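; Elevator actor that moves vertically between a start and an end position when its subida (up) or bajada (down) events are called.
; After a short delay, each event sets a signed spin value on a referenced GiroGiro object, triggers it, then plays a timeline.
; The timelines lerp only the Z height, keeping start X and Y, and update the up/down state flags, which begin as down.
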(event `self.ReceiveTick`
  (params (DeltaSeconds :type "Float (single-precision)")))

(event `self.ReceiveBeginPlay`
  (set `self.EstoyArriba` false)
  (set `self.EstoyAbajo` true))

(event `subida`
  (bind (_posicioninicialsubida_x _posicioninicialsubida_y _posicioninicialsubida_z) (`KismetMathLibrary.BreakVector` (`self.PosicionInicialSubida`)))
  (bind (_posicionfinalsubida_x _posicionfinalsubida_y _posicionfinalsubida_z) (`KismetMathLibrary.BreakVector` (`self.PosicionFinalSubida`)))
  (bind _refgirogiro (`self.RefGiroGiro`))
  (`KismetSystemLibrary.Delay` 2.0)
  (set `/Game/Krosty/Blueprints/SM_ELEVADOR_ENGRANAJES_Blueprint.NumeroGiro` 69.0 _refgirogiro)
  (`/Game/Krosty/Blueprints/SM_ELEVADOR_ENGRANAJES_Blueprint.GiroGiro` _refgirogiro)
  (bind (_direction _subida) (`Timeline|Timeline` :`NewTime` 1.0 :!via `PlayFromStart`)
    (:`Update`
      (`self.K2_SetActorLocation` (`KismetMathLibrary.MakeVector` _posicioninicialsubida_x _posicioninicialsubida_y (`KismetMathLibrary.Lerp` _posicioninicialsubida_z _posicionfinalsubida_z _subida)))
      (set `self.EstoyArriba` true)
      (set `self.EstoyAbajo` false))))

(event `bajada`
  (bind _refgirogiro (`self.RefGiroGiro`))
  (bind (_posicioninicialsubida_x _posicioninicialsubida_y _posicioninicialsubida_z) (`KismetMathLibrary.BreakVector` (`self.PosicionInicialSubida`)))
  (bind (_posicionfinalsubida_x _posicionfinalsubida_y _posicionfinalsubida_z) (`KismetMathLibrary.BreakVector` (`self.PosicionFinalSubida`)))
  (`KismetSystemLibrary.Delay` 2.0)
  (set `/Game/Krosty/Blueprints/SM_ELEVADOR_ENGRANAJES_Blueprint.NumeroGiro` -69.0 _refgirogiro)
  (`/Game/Krosty/Blueprints/SM_ELEVADOR_ENGRANAJES_Blueprint.GiroGiro` _refgirogiro)
  (bind (_direction _subida) (`Timeline|Timeline_0` :`NewTime` 1.0 :!via `PlayFromStart`)
    (:`Update`
      (`self.K2_SetActorLocation` (`KismetMathLibrary.MakeVector` _posicioninicialsubida_x _posicioninicialsubida_y (`KismetMathLibrary.Lerp` _posicionfinalsubida_z _posicioninicialsubida_z _subida)))
      (set `self.EstoyAbajo` true)
      (set `self.EstoyArriba` false))))

(fn `UserConstructionScript`)