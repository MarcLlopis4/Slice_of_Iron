(event `self.ReceiveBeginPlay`
  (bind _inventorywidget (`self.InventoryWidget`))
  (bind _returnvalue (`|CreateWidget` "/Game/Krosty/Inventory/Widgets/WB_Inventory.WB_Inventory_C" (`GameplayStatics.GetPlayerController` 0)))
  (set `self.InventoryWidget` _returnvalue)
  (`KismetArrayLibrary.Array_Resize` (`self.ItemsMateriales`) 30)
  (`/Game/Krosty/Inventory/Widgets/WB_Inventory.LoadInventoryMateriales` _inventorywidget self true 0)
  (`KismetArrayLibrary.Array_Resize` (`self.ItemsArmas`) 5)
  (`/Game/Krosty/Inventory/Widgets/WB_Inventory.LoadInventoryArmas` _inventorywidget self true 0)
  (`KismetArrayLibrary.Array_Resize` (`self.ItemsArmaduras`) 10)
  (`/Game/Krosty/Inventory/Widgets/WB_Inventory.LoadInventoryArmaduras` _inventorywidget self true 0)
  (`KismetArrayLibrary.Array_Resize` (`self.ItemsPartesArmas`) 20)
  (`/Game/Krosty/Inventory/Widgets/WB_Inventory.LoadInventoryPartesArmas` _inventorywidget self true 0)
  (`KismetArrayLibrary.Array_Resize` (`self.ItemsObjetosClave`) 15)
  (`/Game/Krosty/Inventory/Widgets/WB_Inventory.LoadInventoryObjetosClave` _inventorywidget self true 0)
  (`KismetArrayLibrary.Array_Resize` (`self.HotBarWeapons`) 3)
  (`/Game/Krosty/Inventory/Widgets/WB_Inventory.LoadWepaonsHotBar` _inventorywidget self true 0))

(event `Key|I`
  (params (Key :type "Key Structure"))
  (bind _returnvalue (`GameplayStatics.GetPlayerController` 0))
  (bind _inventorywidget (`self.InventoryWidget`))
  (:`Pressed`
    (if (`/Game/Krosty/Inventory/Widgets/WB_Inventory.Showing` (`self.InventoryWidget`))
      (set `PlayerController.bShowMouseCursor` false _returnvalue)
      (`WidgetBlueprintLibrary.SetInputMode_GameOnly` _returnvalue)
      (`/Game/Krosty/Inventory/Widgets/WB_Inventory.ShowInventory` (`self.InventoryWidget`) false)
      (else
        (set `PlayerController.bShowMouseCursor` true (`GameplayStatics.GetPlayerController` 0))
        (`WidgetBlueprintLibrary.SetInputMode_GameAndUIEx` _returnvalue null)
        (`UserWidget.AddToViewport` _inventorywidget 0)
        (`/Game/Krosty/Inventory/Widgets/WB_Inventory.ShowInventory` _inventorywidget true)))))

(event `Key|E`
  (params (Key :type "Key Structure"))
  (bind _itemsmateriales (`self.ItemsMateriales`))
  (bind _itemspartesarmas (`self.ItemsPartesArmas`))
  (bind _itemsarmas (`self.ItemsArmas`))
  (bind _itemsarmaduras (`self.ItemsArmaduras`))
  (bind _itemsobjetosclave (`self.ItemsObjetosClave`))
  (bind _returnvalue (- (`Actor.K2_GetActorLocation` (`GameplayStatics.GetPlayerCharacter` 0)) (0.0 0.0 65.0)))
  (:`Pressed`
    (bind (_outhit _returnvalue_2) (`KismetSystemLibrary.SphereTraceSingle` :`Start` _returnvalue :`End` _returnvalue :`Radius` 360.0 :`TraceChannel` "TraceTypeQuery1" :`DrawDebugType` "Persistent"))
    (if _returnvalue_2
      (bind (_bblockinghit _binitialoverlap _time _distance _location _impactpoint _normal _impactnormal _physmat _hitactor) (`GameplayStatics.BreakHitResult` _outhit))
      (switch `string` (`KismetStringLibrary.Conv_NameToString` (`|GetArrayItem` (`Actor.Tags` _hitactor)))
        (:`ItemMateriales`
          (bind _asbp_item_material (cast `/Game/Krosty/Inventory/Blueprints/BP_ItemMaterial` _hitactor))
          (set `self.itemSet` false)
          (for (_array_element _array_index) _itemsmateriales
            (bind (_name _stackable _quantity) (break `/Game/Krosty/Inventory/Blueprints/S_ItemMaterialStruct` _array_element))
            (bind (_name_2 _stackable_2 _quantity_2) (break `/Game/Krosty/Inventory/Blueprints/S_ItemMaterialStruct` (`/Game/Krosty/Inventory/Blueprints/BP_ItemMaterial.InfoItemMaterial` _asbp_item_material)))
            (if (`KismetTextLibrary.EqualEqual_TextText` _name _name_2)
              (bind _returnvalue_3 (+ _quantity _quantity_2))
              (if (and _stackable_2 (<= _returnvalue_3 64))
                (bind (_infoitemmaterial_name _infoitemmaterial_stackable _infoitemmaterial_quantity _infoitemmaterial_thumnail _infoitemmaterial_mesh) (break `/Game/Krosty/Inventory/Blueprints/S_ItemMaterialStruct` (`/Game/Krosty/Inventory/Blueprints/BP_ItemMaterial.InfoItemMaterial` _asbp_item_material)))
                (`KismetArrayLibrary.Array_Set` (`self.ItemsMateriales`) _array_index (make `/Game/Krosty/Inventory/Blueprints/S_ItemMaterialStruct` _infoitemmaterial_name _infoitemmaterial_stackable _returnvalue_3 _infoitemmaterial_thumnail _infoitemmaterial_mesh))
                (`/Game/Krosty/Inventory/Widgets/WB_Inventory.LoadInventoryMateriales` (`self.InventoryWidget`) self false _array_index)
                (`Actor.K2_DestroyActor` _asbp_item_material)
                (set `self.itemSet` true)
                (break))))
          (if (not (`self.itemSet`))
            (for (_array_element_2 _array_index_2) _itemsmateriales
              (if (== (`.Quantity_13_28028BEF44C31620A0E3EEA07037C568` (break `/Game/Krosty/Inventory/Blueprints/S_ItemMaterialStruct` _array_element_2)) 0)
                (`KismetArrayLibrary.Array_Set` (`self.ItemsMateriales`) _array_index_2 (`/Game/Krosty/Inventory/Blueprints/BP_ItemMaterial.InfoItemMaterial` _asbp_item_material))
                (`/Game/Krosty/Inventory/Widgets/WB_Inventory.LoadInventoryMateriales` (`self.InventoryWidget`) self false _array_index_2)
                (`Actor.K2_DestroyActor` _asbp_item_material)
                (break)))
            (`KismetSystemLibrary.PrintString` "NO space for Materials")))
        (:`ItemPartesArmas`
          (bind _asbp_item_partes_armas (cast `/Game/Krosty/Inventory/Blueprints/BP_ItemPartesArmas` _hitactor))
          (set `self.itemSet` false)
          (for (_array_element_3 _array_index_3) _itemspartesarmas
            (bind (_name_3 _stackable_3 _quantity_3) (break `/Game/Krosty/Inventory/Blueprints/S_PartesArmasStruct` _array_element_3))
            (bind (_name_4 _stackable_4 _quantity_4) (break `/Game/Krosty/Inventory/Blueprints/S_PartesArmasStruct` (`/Game/Krosty/Inventory/Blueprints/BP_ItemPartesArmas.InfoItemPartesArmas` _asbp_item_partes_armas)))
            (if (`KismetTextLibrary.EqualEqual_TextText` _name_3 _name_4)
              (bind _returnvalue_4 (+ _quantity_3 _quantity_4))
              (if (and _stackable_4 (<= _returnvalue_4 64))
                (bind (_infoitempartesarmas_name _infoitempartesarmas_stackable _infoitempartesarmas_quantity _infoitempartesarmas_type _infoitempartesarmas_thumnail _infoitempartesarmas_mesh) (break `/Game/Krosty/Inventory/Blueprints/S_PartesArmasStruct` (`/Game/Krosty/Inventory/Blueprints/BP_ItemPartesArmas.InfoItemPartesArmas` _asbp_item_partes_armas)))
                (`KismetArrayLibrary.Array_Set` (`self.ItemsPartesArmas`) _array_index_3 (make `/Game/Krosty/Inventory/Blueprints/S_PartesArmasStruct` _infoitempartesarmas_name _infoitempartesarmas_stackable _returnvalue_4 "NewEnumerator0" _infoitempartesarmas_thumnail _infoitempartesarmas_mesh "" (struct)))
                (`/Game/Krosty/Inventory/Widgets/WB_Inventory.LoadInventoryPartesArmas` (`self.InventoryWidget`) self false _array_index_3)
                (`Actor.K2_DestroyActor` _asbp_item_partes_armas)
                (set `self.itemSet` true)
                (break))))
          (if (not (`self.itemSet`))
            (for (_array_element_4 _array_index_4) _itemspartesarmas
              (if (== (`.Quantity_13_28028BEF44C31620A0E3EEA07037C568` (break `/Game/Krosty/Inventory/Blueprints/S_PartesArmasStruct` _array_element_4)) 0)
                (`KismetArrayLibrary.Array_Set` (`self.ItemsPartesArmas`) _array_index_4 (`/Game/Krosty/Inventory/Blueprints/BP_ItemPartesArmas.InfoItemPartesArmas` _asbp_item_partes_armas))
                (`/Game/Krosty/Inventory/Widgets/WB_Inventory.LoadInventoryPartesArmas` (`self.InventoryWidget`) self false _array_index_4)
                (`KismetSystemLibrary.PrintString` "parte aram set")
                (`Actor.K2_DestroyActor` _asbp_item_partes_armas)
                (break)))
            (`KismetSystemLibrary.PrintString` "NO space for PartesArmas")))
        (:`ItemArmas`
          (bind _asbp_item_armas (cast `/Game/Krosty/Inventory/Blueprints/BP_ItemArmas` _hitactor))
          (set `self.itemSet` false)
          (for (_array_element_5 _array_index_5) _itemsarmas
            (bind (_name_5 _stackable_5 _quantity_5) (break `/Game/Krosty/Inventory/Blueprints/S_ArmasStruct` _array_element_5))
            (bind (_name_6 _stackable_6 _quantity_6) (break `/Game/Krosty/Inventory/Blueprints/S_ArmasStruct` (`/Game/Krosty/Inventory/Blueprints/BP_ItemArmas.InfoItemArmas` _asbp_item_armas)))
            (if (`KismetTextLibrary.EqualEqual_TextText` _name_5 _name_6)
              (bind _returnvalue_5 (+ _quantity_5 _quantity_6))
              (if (and _stackable_6 (<= _returnvalue_5 64))
                (bind (_infoitemarmas_name _infoitemarmas_stackable _infoitemarmas_quantity _infoitemarmas_thumnail _infoitemarmas_mesh) (break `/Game/Krosty/Inventory/Blueprints/S_ArmasStruct` (`/Game/Krosty/Inventory/Blueprints/BP_ItemArmas.InfoItemArmas` _asbp_item_armas)))
                (`KismetArrayLibrary.Array_Set` (`self.ItemsArmas`) _array_index_5 (make `/Game/Krosty/Inventory/Blueprints/S_ArmasStruct` _infoitemarmas_name _infoitemarmas_stackable _returnvalue_5 _infoitemarmas_thumnail _infoitemarmas_mesh "" (struct)))
                (`/Game/Krosty/Inventory/Widgets/WB_Inventory.LoadInventoryArmas` (`self.InventoryWidget`) self false _array_index_5)
                (`Actor.K2_DestroyActor` _asbp_item_armas)
                (set `self.itemSet` true)
                (break))))
          (if (not (`self.itemSet`))
            (for (_array_element_6 _array_index_6) _itemsarmas
              (if (== (`.Quantity_13_28028BEF44C31620A0E3EEA07037C568` (break `/Game/Krosty/Inventory/Blueprints/S_ArmasStruct` _array_element_6)) 0)
                (`KismetArrayLibrary.Array_Set` (`self.ItemsArmas`) _array_index_6 (`/Game/Krosty/Inventory/Blueprints/BP_ItemArmas.InfoItemArmas` _asbp_item_armas))
                (`/Game/Krosty/Inventory/Widgets/WB_Inventory.LoadInventoryArmas` (`self.InventoryWidget`) self false _array_index_6)
                (`Actor.K2_DestroyActor` _asbp_item_armas)
                (break)))
            (`KismetSystemLibrary.PrintString` "NO space for armas")))
        (:`ItemArmaduras`
          (bind _asbp_item_armaduras (cast `/Game/Krosty/Inventory/Blueprints/BP_ItemArmaduras` _hitactor))
          (set `self.itemSet` false)
          (for (_array_element_7 _array_index_7) _itemsarmaduras
            (bind (_name_7 _stackable_7 _quantity_7) (break `/Game/Krosty/Inventory/Blueprints/S_ArmadurasStruct` _array_element_7))
            (bind (_name_8 _stackable_8 _quantity_8) (break `/Game/Krosty/Inventory/Blueprints/S_ArmadurasStruct` (`/Game/Krosty/Inventory/Blueprints/BP_ItemArmaduras.InfoItemArmaduras` _asbp_item_armaduras)))
            (if (`KismetTextLibrary.EqualEqual_TextText` _name_7 _name_8)
              (bind _returnvalue_6 (+ _quantity_7 _quantity_8))
              (if (and _stackable_8 (<= _returnvalue_6 64))
                (bind (_infoitemarmaduras_name _infoitemarmaduras_stackable _infoitemarmaduras_quantity _infoitemarmaduras_thumnail _infoitemarmaduras_mesh) (break `/Game/Krosty/Inventory/Blueprints/S_ArmadurasStruct` (`/Game/Krosty/Inventory/Blueprints/BP_ItemArmaduras.InfoItemArmaduras` _asbp_item_armaduras)))
                (`KismetArrayLibrary.Array_Set` (`self.ItemsArmaduras`) _array_index_7 (make `/Game/Krosty/Inventory/Blueprints/S_ArmadurasStruct` _infoitemarmaduras_name _infoitemarmaduras_stackable _returnvalue_6 _infoitemarmaduras_thumnail _infoitemarmaduras_mesh))
                (`/Game/Krosty/Inventory/Widgets/WB_Inventory.LoadInventoryArmaduras` (`self.InventoryWidget`) self false _array_index_7)
                (`Actor.K2_DestroyActor` _asbp_item_armaduras)
                (set `self.itemSet` true)
                (break))))
          (if (not (`self.itemSet`))
            (for (_array_element_8 _array_index_8) _itemsarmaduras
              (if (== (`.Quantity_13_28028BEF44C31620A0E3EEA07037C568` (break `/Game/Krosty/Inventory/Blueprints/S_ArmadurasStruct` _array_element_8)) 0)
                (`KismetArrayLibrary.Array_Set` (`self.ItemsArmaduras`) _array_index_8 (`/Game/Krosty/Inventory/Blueprints/BP_ItemArmaduras.InfoItemArmaduras` _asbp_item_armaduras))
                (`/Game/Krosty/Inventory/Widgets/WB_Inventory.LoadInventoryArmaduras` (`self.InventoryWidget`) self false _array_index_8)
                (`Actor.K2_DestroyActor` _asbp_item_armaduras)
                (break)))
            (`KismetSystemLibrary.PrintString` "NO space for armaduras")))
        (:`ItemObjetosClave`
          (bind _asbp_item_objetos_clave (cast `/Game/Krosty/Inventory/Blueprints/BP_ItemObjetosClave` _hitactor))
          (set `self.itemSet` false)
          (for (_array_element_9 _array_index_9) _itemsobjetosclave
            (bind (_name_9 _stackable_9 _quantity_9) (break `/Game/Krosty/Inventory/Blueprints/S_ObjetosClaveStruct` _array_element_9))
            (bind (_name_10 _stackable_10 _quantity_10) (break `/Game/Krosty/Inventory/Blueprints/S_ObjetosClaveStruct` (`/Game/Krosty/Inventory/Blueprints/BP_ItemObjetosClave.InfoItemObjetosClave` _asbp_item_objetos_clave)))
            (if (`KismetTextLibrary.EqualEqual_TextText` _name_9 _name_10)
              (bind _returnvalue_7 (+ _quantity_9 _quantity_10))
              (if (and _stackable_10 (<= _returnvalue_7 64))
                (bind (_infoitemobjetosclave_name _infoitemobjetosclave_stackable _infoitemobjetosclave_quantity _infoitemobjetosclave_thumnail _infoitemobjetosclave_mesh) (break `/Game/Krosty/Inventory/Blueprints/S_ObjetosClaveStruct` (`/Game/Krosty/Inventory/Blueprints/BP_ItemObjetosClave.InfoItemObjetosClave` _asbp_item_objetos_clave)))
                (`KismetArrayLibrary.Array_Set` (`self.ItemsObjetosClave`) _array_index_9 (make `/Game/Krosty/Inventory/Blueprints/S_ObjetosClaveStruct` _infoitemobjetosclave_name _infoitemobjetosclave_stackable _returnvalue_7 _infoitemobjetosclave_thumnail _infoitemobjetosclave_mesh))
                (`/Game/Krosty/Inventory/Widgets/WB_Inventory.LoadInventoryObjetosClave` (`self.InventoryWidget`) self false _array_index_9)
                (`Actor.K2_DestroyActor` _asbp_item_objetos_clave)
                (set `self.itemSet` true)
                (break))))
          (if (not (`self.itemSet`))
            (for (_array_element_10 _array_index_10) _itemsobjetosclave
              (if (== (`.Quantity_13_28028BEF44C31620A0E3EEA07037C568` (break `/Game/Krosty/Inventory/Blueprints/S_ObjetosClaveStruct` _array_element_10)) 0)
                (`KismetArrayLibrary.Array_Set` (`self.ItemsObjetosClave`) _array_index_10 (`/Game/Krosty/Inventory/Blueprints/BP_ItemObjetosClave.InfoItemObjetosClave` _asbp_item_objetos_clave))
                (`/Game/Krosty/Inventory/Widgets/WB_Inventory.LoadInventoryObjetosClave` (`self.InventoryWidget`) self false _array_index_10)
                (`Actor.K2_DestroyActor` _asbp_item_objetos_clave)
                (break)))
            (`KismetSystemLibrary.PrintString` "NO space for ObjetosClave")))))))